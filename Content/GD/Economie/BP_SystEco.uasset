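; BP_SystEco is the economy system that tracks the player's money, displayed as crystals, and registers itself on BP_ThirdPersonGameMode at BeginPlay.
; GagnerArgent adds to the target balance, shows the money HUD and uses a timeline lerp to count the displayed amount up, hiding it when finished.
; Payer deducts a price only if AssezDeThunes confirms the target balance covers it, without animation or widget refresh.
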(event EventBeginPlay
  (bind _asbp_third_person_game_mode (Utilities|Casting|CastToBP_ThirdPersonGameMode (Game|GetGameMode)))
  (Variables|/Game/GD/GameMode/Blueprints/BP_ThirdPersonGameMode.BP_ThirdPersonGameMode_C|SetSystemeEco _asbp_third_person_game_mode self)
  (Variables|Default|SetGM _asbp_third_person_game_mode))

(event EventGagnerArgent
  (params (ArgentGagner :type Integer))
  (if (not (== ArgentGagner 0))
    (Default|AfficheMoneyCollectible (Variables|Default|GetGM) true "Visible")
    (Variables|Default|SetArgentActuel (Variables|Default|GetArgentTarget))
    (Variables|Default|SetArgentTarget (+ ArgentGagner (Variables|Default|GetArgentTarget)))
    (bind _newtrack_0 (Timeline|Timeline PlayFromStart)
      (:Update
        (bind _output_get (Variables|Default|SetArgentAfficheAuJoueur (Math|Float|Truncate (Math|Float|Lerp (Math|Conversions|ToFloat(Integer) (Variables|Default|GetArgentActuel)) (Math|Conversions|ToFloat(Integer) (Variables|Default|GetArgentTarget)) _newtrack_0))))
        (Rendering|Components|TextRender|SetText (Variables|/Game/GD/UI/WB_MainGame.WB_MainGame_C|GetRichText_Cristaux (Variables|/Game/GD/GameMode/Blueprints/BP_ThirdPersonGameMode.BP_ThirdPersonGameMode_C|GetWidgetMainGame (Variables|Default|GetGM))) (Utilities|Text|ToText(Integer) _output_get)))
      (:Finished
        (Variables|Default|SetArgentActuel (Variables|Default|GetArgentTarget))
        (Default|AfficheMoneyCollectible (Variables|Default|GetGM) true "Hidden")))))

(event EventPayer
  (params (Prix :type Integer))
  (bind _assezdethune (CallFunction|AssezDeThunes Prix))
  (if _assezdethune
    (Variables|Default|SetArgentActuel (Variables|Default|GetArgentTarget))
    (bind _output_get (Variables|Default|SetArgentTarget (- (Variables|Default|GetArgentTarget) Prix)))
    (Variables|Default|SetArgentAfficheAuJoueur _output_get)))

(fn ConstructionScript)

(fn AssezDeThunes
  (params (PrixAPayer :type Integer))
  (return (<= PrixAPayer (Variables|Default|GetArgentTarget))))