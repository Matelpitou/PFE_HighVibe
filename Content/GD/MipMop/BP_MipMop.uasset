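; MipMop is an actor that follows the player character, a BP_PP_Yass cached on BeginPlay.
; Each Tick it turns on yaw to face the player and, unless closer than 200 units, steps along its root's forward vector.
; Movement sets the location directly without sweep, using a fixed step per frame that is not scaled by delta time.
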(event EventBeginPlay
  (bind _asbp_pp_yass (Utilities|Casting|CastToBP_PP_Yass (Game|GetPlayerCharacter 0)))
  (Variables|Default|SetPlayer _asbp_pp_yass))

(event EventTick
  (params (DeltaSeconds :type Float%20%28single-precision%29))
  (Transformation|SetActorRotation (Math|Rotator|MakeRotator 0.0 0.0 (.yaw (Math|Rotator|FindLookatRotation (Transformation|GetActorLocation) (Transformation|GetActorLocation (Variables|Default|GetPlayer))))))
  (if (not (< (Transformation|GetDistanceTo (Variables|Default|GetPlayer)) 2e+02))
    (Transformation|SetActorLocation (+ (* (Math|Vector|GetForwardVector (Variables|Default|GetDefaultSceneRoot self)) 5) (Transformation|GetActorLocation)) false false)))

(fn ConstructionScript)