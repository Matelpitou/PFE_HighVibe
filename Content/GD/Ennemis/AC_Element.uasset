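; Enemy component that displays the electricity and water counts on its BP_Enn_EnnParent owner.
; SetElec destroys the previous markers, then attaches one BP_Elec or BP_Eau actor per count, showing that element's symbol instead at its max.
; All markers share the AllWater array and are spaced evenly in a ring around the enemy.
; The electric symbol's visibility stays unchanged while stunned, and Die clears all markers.
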(event Custom|SetElec
  (params (NewElecCount :type Integer) (NewWaterCount :type Integer) (MaxElec :type Integer) (MaxEau :type Integer))
  (bind _returnvalue (>= NewWaterCount MaxEau))
  (bind _returnvalue_2 (>= NewElecCount MaxElec))
  (bind _allwater (Variables|Default|GetAllWater))
  (bind _allwater_2 (Variables|Default|GetAllWater))
  (bind _as_bp_enn_enn_parent (Variables|Default|GetAs%20BP%20Enn%20Enn%20Parent))
  (bind _returnvalue_3 (Utilities|Array|Length _allwater_2))
  (for _array_element _allwater
    (Actor|DestroyActor _array_element))
  (Utilities|Array|Clear _allwater)
  (if (Variables|/Game/GD/Ennemis/Cac/BP_Enn_EnnParent.BP_Enn_EnnParent_C|GetStunn _as_bp_enn_enn_parent)
    _
    (else
      (Development|SetHiddeninGame (Variables|/Game/GD/Ennemis/Cac/BP_Enn_EnnParent.BP_Enn_EnnParent_C|GetElecSymbol _as_bp_enn_enn_parent) (not _returnvalue_2) false)))
  (if _returnvalue_2
    _
    (else
      (for _index (range 0 (- NewElecCount 1))
        ;[1 1 1] SpawnElec
        (bind _returnvalue_4 (Game|SpawnActorfromClass "/Game/GD/Ennemis/BP_Elec.BP_Elec_C" (Transformation|GetActorTransform (Components|GetOwner)) "Undefined" "MultiplyWithRoot" 0 0))
        (bind _output_get (Variables|Default|SetSpawnedElec _returnvalue_4))
        (Transformation|AttachActorToActor _output_get (Components|GetOwner) "None" "SnapToTarget" "KeepWorld" "KeepRelative" true)
        (Utilities|Array|Add (Variables|Default|GetAllWater) (Variables|Default|GetSpawnedElec)))))
  (Development|SetHiddeninGame (Variables|/Game/GD/Ennemis/Cac/BP_Enn_EnnParent.BP_Enn_EnnParent_C|GetWaterSymbol (Variables|Default|GetAs%20BP%20Enn%20Enn%20Parent)) (not _returnvalue) false)
  (if _returnvalue
    _
    (else
      (for _index_2 (range 0 (- NewWaterCount 1))
        ;[1 1 1] SpawnEau
        (bind _returnvalue_5 (Game|SpawnActorfromClass "/Game/GD/Ennemis/BP_Eau.BP_Eau_C" (Transformation|GetActorTransform (Components|GetOwner)) "Undefined" "MultiplyWithRoot" 0 0))
        (bind _output_get_2 (Variables|Default|SetSpawnedWater _returnvalue_5))
        (Transformation|AttachActorToActor _output_get_2 (Components|GetOwner) "None" "SnapToTarget" "KeepWorld" "KeepRelative" true)
        (Utilities|Array|Add (Variables|Default|GetAllWater) (Variables|Default|GetSpawnedWater)))))
  ;[1 1 1] Les ranger
  (for _index_3 (range 0 (- _returnvalue_3 1))
    (Transformation|SetActorRelativeRotation (Utilities|Array|Get(acopy) (Variables|Default|GetAllWater) _index_3) (Math|Rotator|MakeRotator 0.0 0.0 (Math|Conversions|ToFloat(Integer) (* (/ 360 _returnvalue_3) _index_3))))
    (Transformation|SetActorRelativeLocation (Utilities|Array|Get(acopy) (Variables|Default|GetAllWater) _index_3) (Math|Vector|MakeVector (.x (* (Math|Vector|GetForwardVector (Transformation|GetActorRotation (Utilities|Array|Get(acopy) (Variables|Default|GetAllWater) _index_3))) 20)) (.y (* (Math|Vector|GetForwardVector (Transformation|GetActorRotation (Utilities|Array|Get(acopy) (Variables|Default|GetAllWater) _index_3))) 20)) (+ (.z (Transformation|GetActorLocation (Utilities|Array|Get(acopy) (Variables|Default|GetAllWater) _index_3))) 5.0)))))

(event Custom|Die
  (bind _allwater (Variables|Default|GetAllWater))
  (for _array_element _allwater
    (Actor|DestroyActor _array_element))
  (Utilities|Array|Clear _allwater))

(event EventBeginPlay
  (bind _asbp_enn_enn_parent (Utilities|Casting|CastToBP_Enn_EnnParent (Components|GetOwner)))
  (Variables|Default|SetAs%20BP%20Enn%20Enn%20Parent _asbp_enn_enn_parent))