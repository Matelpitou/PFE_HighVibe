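; Spawner for BP_Enn_Dist enemies that places them around itself at random reachable points within a radius.
; With FromBeginning, enemies spawn at BeginPlay with economy and crowd manager references, then attack on trigger in Crazy state if Libre is set.
; Otherwise the trigger spawns them already Crazy and attacking, without a crowd manager.
; The trigger fires once, from ForceSpawn or BP_PP_Yass entering the box unless Desactiver is set.
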(event OnComponentBeginOverlap(Box)
  (params (OverlappedComponent :type Primitive%20Component%20Object%20Reference) (OtherActor :type Actor%20Object%20Reference) (OtherComp :type Primitive%20Component%20Object%20Reference) (OtherBodyIndex :type Integer) (bFromSweep :type Boolean) (SweepResult :type Hit%20Result%20Structure%20%28by%20ref%29))
  (if (not (Variables|Default|GetDesactiver))
    (Utilities|Casting|CastToBP_PP_Yass OtherActor)
    (Utilities|FlowControl|DoOnce false
      (:Completed
        (if (Variables|Default|GetFromBeginning)
          (for _array_element (Variables|Default|GetTempEnnSpawned)
            (if (Variables|Default|GetLibre)
              (Variables|/Game/GD/Ennemis/Cac/BP_Enn_EnnParent.BP_Enn_EnnParent_C|SetCrazy _array_element true)
              (Default|GoAttack1 _array_element)))
          (else
            (for _index (range 0 (Variables|Default|GetEnnemiNumber))
              (bind _returnvalue (CallFunction|SpawnEnnDist))
              (Variables|/Game/GD/Ennemis/Cac/BP_Enn_EnnParent.BP_Enn_EnnParent_C|SetCrazy _returnvalue true)
              (Variables|/Game/GD/Ennemis/Cac/BP_Enn_EnnParent.BP_Enn_EnnParent_C|SetSystEco _returnvalue (Variables|Default|GetSystEco))
              (Default|GoAttack1 _returnvalue))))))))

(event Custom|ForceSpawn
  (Utilities|FlowControl|DoOnce false
    (:Completed
      (if (Variables|Default|GetFromBeginning)
        (for _array_element (Variables|Default|GetTempEnnSpawned)
          (if (Variables|Default|GetLibre)
            (Variables|/Game/GD/Ennemis/Cac/BP_Enn_EnnParent.BP_Enn_EnnParent_C|SetCrazy _array_element true)
            (Default|GoAttack1 _array_element)))
        (else
          (for _index (range 0 (Variables|Default|GetEnnemiNumber))
            (bind _returnvalue (CallFunction|SpawnEnnDist))
            (Variables|/Game/GD/Ennemis/Cac/BP_Enn_EnnParent.BP_Enn_EnnParent_C|SetCrazy _returnvalue true)
            (Variables|/Game/GD/Ennemis/Cac/BP_Enn_EnnParent.BP_Enn_EnnParent_C|SetSystEco _returnvalue (Variables|Default|GetSystEco))
            (Default|GoAttack1 _returnvalue)))))))

(event EventBeginPlay
  (if (Variables|Default|GetFromBeginning)
    (for _index (range 0 (Variables|Default|GetEnnemiNumber))
      (bind _returnvalue (CallFunction|SpawnEnnDist))
      (Utilities|Array|Add (Variables|Default|GetTempEnnSpawned) _returnvalue)
      (Variables|/Game/GD/Ennemis/Cac/BP_Enn_EnnParent.BP_Enn_EnnParent_C|SetSystEco _returnvalue (Variables|Default|GetSystEco))
      (Variables|/Game/GD/Ennemis/Enn_Dist/BP_Enn_Dist.BP_Enn_Dist_C|SetCrowdManager _returnvalue (Variables|Default|GetReferent)))))

(fn ConstructionScript)

(fn SpawnEnnDist
  (bind _returnvalue (Transformation|GetActorLocation))
  (bind _spawnradius (Variables|Default|GetSpawnRadius))
  (bind _randomlocation (AI|Navigation|GetRandomReachablePointinRadius _returnvalue _spawnradius 0 0))
  (bind _returnvalue_2 (Game|SpawnActorfromClass "/Game/GD/Ennemis/Enn_Dist/BP_Enn_Dist.BP_Enn_Dist_C" (Math|Transform|MakeTransform (Math|Vector|MakeVector (.x _randomlocation) (.y _randomlocation) (+ (.z (Transformation|GetActorLocation)) 1e+01)) "0, 0, 0" "1.000000,1.000000,1.000000") "AdjustIfPossibleButAlwaysSpawn" "MultiplyWithRoot" 0 0))
  (return _returnvalue_2))