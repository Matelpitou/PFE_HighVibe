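; Ranged enemy projectile that launches its sphere toward the player's position at spawn and telegraphs the landing spot.
; BeginPlay derives a forward impulse from the distance to the player using a ballistic range-style formula, then spawns a BP_CircleProjectile marker at the player's mesh.
; A looping timer grows the marker's red center as the sphere nears the saved position.
; Any sphere overlap destroys both marker and projectile, without applying damage.
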(event OnComponentBeginOverlap(Sphere)
  (params (OverlappedComponent :type Primitive%20Component%20Object%20Reference) (OtherActor :type Actor%20Object%20Reference) (OtherComp :type Primitive%20Component%20Object%20Reference) (OtherBodyIndex :type Integer) (bFromSweep :type Boolean) (SweepResult :type Hit%20Result%20Structure%20%28by%20ref%29))
  (Development|PrintString "Hello")
  (CallFunction|Blow))

(event Custom|Blow
  (Actor|DestroyActor (Variables|Default|GetSpawnedCircle))
  (Actor|DestroyActor))

(event Custom|MajCircle
  (bind _sphere (Variables|Default|GetSphere))
  (bind _totaldistance (Variables|Default|GetTotalDistance))
  (bind _playerbaselocation (Variables|Default|GetPlayerBaseLocation))
  (bind _returnvalue (Transformation|GetWorldLocation _sphere))
  (bind _returnvalue_2 (Math|Vector|Distance(Vector) _playerbaselocation _returnvalue))
  (bind _returnvalue_3 (/ _returnvalue_2 _totaldistance))
  (bind _returnvalue_4 (Math|Float|Lerp 1.55 0.0 _returnvalue_3))
  (Transformation|SetWorldScale3D (Variables|/Game/GD/Ennemis/Enn_Dist/BP_CircleProjectile.BP_CircleProjectile_C|GetCenterRed (Variables|Default|GetSpawnedCircle)) (Math|Vector|MakeVector _returnvalue_4 _returnvalue_4 0.02)))

(event Custom|SpawnCircle
  (bind _returnvalue (Game|SpawnActorfromClass "/Game/GD/Ennemis/Enn_Dist/BP_CircleProjectile.BP_CircleProjectile_C" (Math|Transform|MakeTransform (Transformation|GetWorldLocation (Variables|/Script/Engine.Character|GetMesh (Variables|Default|GetAs%20BP%20PP%20Yass))) "0, 0, 0" "1.000000,1.000000,1.000000") "Undefined" "MultiplyWithRoot" 0 0))
  (Variables|Default|SetSpawnedCircle _returnvalue)
  (Utilities|Time|SetTimerbyEvent (delegate Custom|MajCircle) (Utilities|Time|GetWorldDeltaSeconds) true))

(event EventBeginPlay
  (bind _sphere (Variables|Default|GetSphere))
  (bind _returnvalue (Transformation|GetWorldLocation _sphere))
  (bind _asbp_pp_yass (Utilities|Casting|CastToBP_PP_Yass (Game|GetPlayerCharacter 0)))
  (Variables|Default|SetAs%20BP%20PP%20Yass _asbp_pp_yass)
  (Variables|Default|SetPlayerBaseLocation (Transformation|GetActorLocation _asbp_pp_yass))
  (Variables|Default|SetProjectileSpawnLocation _returnvalue)
  (Variables|Default|SetTotalDistance (Math|Vector|Distance(Vector) (Transformation|GetActorLocation _asbp_pp_yass) _returnvalue))
  (Physics|AddImpulse (Variables|Default|GetSphere) (* (* (Math|Float|Sqrt (* (/ (Math|Vector|Distance(Vector) (Transformation|GetActorLocation _asbp_pp_yass) _returnvalue) (Math|Trig|Sin(Degrees) 1.2e+02)) 9.81)) 1e+01) (Math|Vector|GetForwardVector (Transformation|GetWorldRotation (Variables|Default|GetDefaultSceneRoot)))) "None" false)
  (CallFunction|SpawnCircle))

(fn ConstructionScript)