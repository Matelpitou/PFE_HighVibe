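; BP_CheckEnnemy runs a two-wave enemy encounter that finishes with the level 1 end cinematic.
; The player's first entry into BoxPP forces wave one into combat and starts a half-second polling loop.
; Enemies leaving BoxEnnemi decrement EnemyMax; at zero, wave two spawns.
; After the last wave, it reveals SkeletalEnd, plays LS_finLV1, switches player mapping and saves coins to the game instance.
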(event OnComponentBeginOverlap(BoxPP)
  (params (OverlappedComponent :type Primitive%20Component%20Object%20Reference) (OtherActor :type Actor%20Object%20Reference) (OtherComp :type Primitive%20Component%20Object%20Reference) (OtherBodyIndex :type Integer) (bFromSweep :type Boolean) (SweepResult :type Hit%20Result%20Structure%20%28by%20ref%29))
  (Utilities|Casting|CastToBP_PP_Yass OtherActor)
  (Utilities|FlowControl|DoOnce false
    (:Completed
      (CallFunction|ActiveSpawn)
      (CallFunction|CheckMax))))

(event OnComponentEndOverlap(BoxEnnemi)
  (params (OverlappedComponent :type Primitive%20Component%20Object%20Reference) (OtherActor :type Actor%20Object%20Reference) (OtherComp :type Primitive%20Component%20Object%20Reference) (OtherBodyIndex :type Integer))
  (Utilities|Casting|CastToBP_Enn_EnnParent OtherActor)
  (bind _result (Math|Integer|DecrementInt (Variables|Default|GetEnemyMax))
    (:%20%20
      (Variables|Default|SetEnemyMax _result))))

(event Custom|Check%20Max
  (Utilities|FlowControl|Delay 0.5)
  (if (<= (Variables|Default|GetEnemyMax) 0)
    (CallFunction|ActiveSpawn (Variables|Default|GetWave?)))
  (CallFunction|CheckMax))

(event Custom|ActiveSpawn
  (params (Wave :type Integer))
  (switch int Wave
    (:0
      (for _array_element (Variables|Default|GetSpawnerCacW1)
        (Default|ForceCombat _array_element))
      (for _array_element_2 (Variables|Default|GetSpawnerDistW1)
        (Default|ForceCombat _array_element_2))
      (Variables|Default|SetEnemyMax (Utilities|Array|Get(acopy) (Variables|Default|GetenemyMaxWave) (Variables|Default|GetWave?)))
      (bind _result (Math|Integer|IncrementInt (Variables|Default|GetWave?))
        (:%20%20
          (Variables|Default|SetWave? _result))))
    (:1
      (Utilities|Array|Clear (Variables|Default|GetTabEnnemie))
      (for _array_element_3 (Variables|Default|GetSpawnerCacW2)
        (Default|ForceSpawntheGuys _array_element_3))
      (for _array_element_4 (Variables|Default|GetSpawnerCacW2)
        (Default|ForceCombat _array_element_4))
      (for _array_element_5 (Variables|Default|GetSpawnerDistW2)
        (Default|ForceSpawntheGuys _array_element_5))
      (for _array_element_6 (Variables|Default|GetSpawnerDistW2)
        (Default|ForceCombat _array_element_6))
      (Variables|Default|SetEnemyMax (Utilities|Array|Get(acopy) (Variables|Default|GetenemyMaxWave) (Variables|Default|GetWave?)))
      (bind _result_2 (Math|Integer|IncrementInt (Variables|Default|GetWave?))
        (:%20%20
          (Variables|Default|SetWave? _result_2))))
    (:2
      (Utilities|FlowControl|DoOnce false
        (:Completed
          (Utilities|FlowControl|Delay 2.0)
          (Rendering|SetVisibility (Variables|/Script/Engine.SkeletalMeshActor|GetSkeletalMeshComponent (Variables|Default|GetSkeletalEnd)) true false)
          (bind _returnvalue (Sequencer|Player|CreateLevelSequencePlayer "/Game/3D/cinematic_lv1/LS_finLV1.LS_finLV1" (Variables|Default|GetSettings)))
          (Sequencer|Player|Play _returnvalue :!class /Script/MovieScene.MovieSceneSequencePlayer)
          (bind _asbp_pp_yass (Utilities|Casting|CastToBP_PP_Yass (Game|GetPlayerCharacter 0)))
          (Default|MappingCineamatique _asbp_pp_yass true)
          (bind _asbp_main_game_instance (Utilities|Casting|CastToBP_MainGameInstance (Game|GetGameInstance)))
          (Variables|/Game/GD/GameMode/Blueprints/BP_MainGameInstance.BP_MainGameInstance_C|SetCoins _asbp_main_game_instance (Variables|/Game/GD/Economie/BP_SystEco.BP_SystEco_C|GetArgentTarget (Variables|Default|GetSystEco))))))))

(event EventBeginPlay
  (Rendering|SetVisibility (Variables|/Script/Engine.SkeletalMeshActor|GetSkeletalMeshComponent (Variables|Default|GetSkeletalEnd)) false false))

(fn ConstructionScript)