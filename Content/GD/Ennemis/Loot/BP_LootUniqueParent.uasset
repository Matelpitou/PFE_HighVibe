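; BP_LootUniqueParent is the base actor for unique loot pickups that hover in the world until the player collects them.
; A timeline started at BeginPlay offsets the actor's Z from its starting location along a curve.
; The first overlap of its box by BP_PP_Yass hides the item mesh and opens a WB_FindLoot widget, passing itself and its display image.
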(event OnComponentBeginOverlap(Box)
  (params (OverlappedComponent :type Primitive%20Component%20Object%20Reference) (OtherActor :type Actor%20Object%20Reference) (OtherComp :type Primitive%20Component%20Object%20Reference) (OtherBodyIndex :type Integer) (bFromSweep :type Boolean) (SweepResult :type Hit%20Result%20Structure%20%28by%20ref%29))
  (Utilities|Casting|CastToBP_PP_Yass OtherActor)
  (Utilities|FlowControl|DoOnce false
    (:Completed
      (Rendering|SetVisibility (Variables|Default|GetItem) false true)
      (bind _returnvalue (UserInterface|CreateWidget "/Game/GD/Ennemis/Loot/WB_FindLoot.WB_FindLoot_C" 0 self))
      (Variables|/Game/GD/Ennemis/Loot/WB_FindLoot.WB_FindLoot_C|SetItemToGive _returnvalue self)
      (Variables|/Game/GD/Ennemis/Loot/WB_FindLoot.WB_FindLoot_C|SetImageToShow _returnvalue (Variables|Default|GetImageToShow))
      (UserInterface|Viewport|AddtoViewport _returnvalue 0))))

(event EventBeginPlay
  (Variables|Default|SetBaseLocation (Transformation|GetActorLocation))
  (bind _newtrack_0 (Timeline|Timeline PlayFromStart)
    (:Update
      (Transformation|SetActorLocation (Math|Vector|MakeVector (.x (Variables|Default|GetBaseLocation)) (.y (Variables|Default|GetBaseLocation)) (+ _newtrack_0 (.z (Variables|Default|GetBaseLocation)))) false false))))

(fn ConstructionScript)