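; BP_LootEnnemis is an enemy loot pickup that homes in on the player automatically once spawned.
; On BeginPlay it caches the BP_PP_Yass player and its own start location, then plays a timeline that lerps it toward the player's current position without sweeping.
; When the timeline finishes, it prints a money-gain debug string and destroys itself; no reward is actually granted here.
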(event EventBeginPlay
  (bind _asbp_pp_yass (Utilities|Casting|CastToBP_PP_Yass (Game|GetPlayerCharacter 0)))
  (bind _output_get (Variables|Default|SetPlayer _asbp_pp_yass))
  (bind _output_get_2 (Variables|Default|SetStartLocation (Transformation|GetActorLocation)))
  (bind _newtrack_0 (Timeline|Timeline PlayFromStart)
    (:Update
      (Utilities|IsValid _output_get
        (:Is%20Valid
          (Transformation|SetActorLocation (Math|Vector|Lerp(Vector) _output_get_2 (Transformation|GetActorLocation _output_get) _newtrack_0) false false))))
    (:Finished
      (Development|PrintString "Gagnerdesthunes")
      (Actor|DestroyActor))))

(event Collision|EventActorBeginOverlap
  (params (OtherActor :type Actor%20Object%20Reference)))

(event EventTick
  (params (DeltaSeconds :type Float%20%28single-precision%29)))

(fn ConstructionScript)