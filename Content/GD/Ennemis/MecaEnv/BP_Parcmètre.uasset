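; BP_Parcmètre is a parking meter that pays out money and loot when it takes damage.
; Each hit credits its value through SystEco, plays a Timeline-driven scale animation and spawns a BP_LootEnnemis just above it.
; HPBarricade counts hits upward and sets the Destroyed flag at its maximum, after which damage is ignored but the actor stays in the world.
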(event EventTakeDamage
  (params (Damage :type Integer) (StackEau :type Integer) (StackElec :type Integer))
  (bind _returnvalue (Transformation|GetActorTransform))
  (if (not (Variables|Default|GetDestroyed))
    (Default|GagnerArgent (Variables|Default|GetSystEco) (Variables|Default|GetValeur))
    (Utilities|FlowControl|Sequence
      (:then_0
        (bind _newtrack_0 (Timeline|Timeline PlayFromStart)
          (:Update
            (Transformation|SetActorScale3D (Math|Vector|MakeVector (.x _newtrack_0) (.y _newtrack_0) (.z _newtrack_0))))))
      (:then_1
        (Game|SpawnActorfromClass "/Game/GD/Ennemis/Loot/BP_LootEnnemis.BP_LootEnnemis_C" (Math|Transform|MakeTransform (Math|Vector|MakeVector (.x (.location _returnvalue)) (.y (.location _returnvalue)) (+ (.z (.location _returnvalue)) 1e+02)) (.rotation _returnvalue) (.scale _returnvalue)) "Undefined" "MultiplyWithRoot" 0 0)
        (bind _output_get (Variables|Default|SetHPBarricade (+ (Variables|Default|GetHPBarricade) 1)))
        (if (== _output_get (Variables|Default|GetHPBarricadeMax))
          (Variables|Default|SetDestroyed true))))))

(fn ConstructionScript
  (|CallParentFunction))