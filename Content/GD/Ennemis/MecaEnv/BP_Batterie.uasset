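; BP_Batterie is an environment battery that charges from electric hits and powers a linked item.
; Each TakeDamage event with a positive StackElec adds one to HPBarricade, which serves as a charge counter despite its name.
; When the counter equals HPBarricadeMax, it messages a valid LinkedItem through BPI_Activer and activates its particle system.
; A gate then closes, so further hits are ignored after a successful activation.
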(event EventTakeDamage
  (params (Damage :type Integer) (StackEau :type Integer) (StackElec :type Integer))
  (bind _linkeditem (Variables|Default|GetLinkedItem))
  (Utilities|FlowControl|Gate false :!label _label
    (:Exit
      (if (> StackElec 0)
        (bind _output_get (Variables|Default|SetHPBarricade (+ (Variables|Default|GetHPBarricade) 1)))
        (if (== (Variables|Default|GetHPBarricadeMax) _output_get)
          (Utilities|IsValid _linkeditem
            (:Is%20Valid
              (if (Utilities|DoesObjectImplementInterface _linkeditem "/Game/GD/Ennemis/MecaEnv/BPI_Activer.BPI_Activer_C")
                (Class|BPIActiver|ActiveTarget(Message) _linkeditem)
                (Components|Activation|SetActive (Variables|Default|GetParticleSystem) true false)
                (goto _label Close)))))))))

(fn ConstructionScript
  (|CallParentFunction))