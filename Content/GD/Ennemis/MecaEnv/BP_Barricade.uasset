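; BP_Barricade is a destructible environment obstacle that can optionally be on fire (Feu), with active particles.
; Hits through TakeDamage increment a hit counter, but a burning barricade only accepts hits carrying water stacks (StackEau).
; Each hit raises AlphaDestruct on dynamic material instances of the High and Low meshes.
; At the maximum, it hides High, disables its collision and stops the particles, leaving Low in place.
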(event EventBeginPlay
  (if (Variables|Default|GetFeu)
    (Components|Activation|SetActive (Variables|Default|GetParticleSystem) true false))
  (bind _returnvalue (Rendering|Material|CreateDynamicMaterialInstance (Variables|Default|GetHigh) 0 "/Game/GD/Ennemis/MecaEnv/MI_Casser.MI_Casser" "None" :!class /Script/Engine.PrimitiveComponent))
  (Variables|Default|SetCubeHighMaterial _returnvalue)
  (bind _returnvalue_2 (Rendering|Material|CreateDynamicMaterialInstance (Variables|Default|GetLow) 0 "/Game/GD/Ennemis/MecaEnv/MI_Casser.MI_Casser" "None" :!class /Script/Engine.PrimitiveComponent))
  (Variables|Default|SetCubeLowMaterial _returnvalue_2))

(event EventTakeDamage
  (params (Damage :type Integer) (StackEau :type Integer) (StackElec :type Integer))
  (bind _returnvalue (Utilities|Name|MakeLiteralName "AlphaDestruct"))
  (bind _high (Variables|Default|GetHigh))
  (if (not (Variables|Default|GetDestroyed))
    (if (Variables|Default|GetFeu)
      (if (> StackEau 0)
        (bind _output_get (Variables|Default|SetHPBarricade (+ (Variables|Default|GetHPBarricade) 1) :!label _label))
        (Rendering|Material|SetScalarParameterValue (Variables|Default|GetCubeHighMaterial) _returnvalue (/ (Math|Conversions|ToFloat(Integer) (Variables|Default|GetHPBarricade)) (Math|Conversions|ToFloat(Integer) (Variables|Default|GetHPBarricadeMax))) :!class /Script/Engine.MaterialInstanceDynamic)
        (Rendering|Material|SetScalarParameterValue (Variables|Default|GetCubeLowMaterial) _returnvalue (/ (Math|Conversions|ToFloat(Integer) (Variables|Default|GetHPBarricade)) (Math|Conversions|ToFloat(Integer) (Variables|Default|GetHPBarricadeMax))) :!class /Script/Engine.MaterialInstanceDynamic)
        (if (== _output_get (Variables|Default|GetHPBarricadeMax))
          (Rendering|SetVisibility _high false false)
          (Collision|SetCollisionEnabled _high "NoCollision")
          (Variables|Default|SetDestroyed true)
          (Components|Activation|SetActive (Variables|Default|GetParticleSystem) false false))
        (else
          (Development|PrintString "inefficace")))
      (else
        (goto _label)))))

(fn ConstructionScript
  (|CallParentFunction))