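; BP_KingOfTheHill is an enemy encounter zone built around child BP_Enn_Spawner actors.
; BeginPlay configures those spawners, splitting the enemy count by child actor count and passing on the Referent.
; The first BP_PP_Yass overlap of the box spawns a dialogue trigger with this actor as its Referent.
; ActiveTarget activates the particle system, then force-spawns every spawner after a delay.
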(event OnComponentBeginOverlap(Box)
  (params (OverlappedComponent :type Primitive%20Component%20Object%20Reference) (OtherActor :type Actor%20Object%20Reference) (OtherComp :type Primitive%20Component%20Object%20Reference) (OtherBodyIndex :type Integer) (bFromSweep :type Boolean) (SweepResult :type Hit%20Result%20Structure%20%28by%20ref%29))
  (bind _asbp_pp_yass (Utilities|Casting|CastToBP_PP_Yass OtherActor))
  (Utilities|FlowControl|DoOnce false
    (:Completed
      (bind _returnvalue (Game|SpawnActorfromClass "/Game/GD/Dialogues/BP_DialogueTrigger.BP_DialogueTrigger_C" (Transformation|GetActorTransform _asbp_pp_yass) "Undefined" "MultiplyWithRoot" 0 0))
      (Variables|/Game/GD/Dialogues/BP_DialogueTrigger.BP_DialogueTrigger_C|SetText _returnvalue (Variables|Default|GetText))
      (Variables|/Game/GD/Dialogues/BP_DialogueTrigger.BP_DialogueTrigger_C|SetMipMop? _returnvalue (Variables|Default|GetMip%20Mop?))
      (Variables|/Game/GD/Dialogues/BP_DialogueTrigger.BP_DialogueTrigger_C|SetReferent _returnvalue self))))

(event EventActiveTarget
  (Components|Activation|SetActive (Variables|Default|GetParticleSystem) true false)
  (Utilities|FlowControl|Delay 4.0)
  (for _array_element (Actor|GetAllChildActors true)
    (bind _asbp_enn_spawner (Utilities|Casting|CastToBP_Enn_Spawner _array_element))
    (Default|ForceSpawn _asbp_enn_spawner)))

(event EventBeginPlay
  (bind _childactors (Actor|GetAllChildActors true))
  (for _array_element _childactors
    (bind _asbp_enn_spawner (Utilities|Casting|CastToBP_Enn_Spawner _array_element))
    (Variables|/Game/GD/Ennemis/BP_Enn_Spawner.BP_Enn_Spawner_C|SetEnnemiNumber _asbp_enn_spawner (/ (Variables|Default|GetEnnemisNumber) (Utilities|Array|Length _childactors)))
    (Variables|/Game/GD/Ennemis/BP_Enn_Spawner.BP_Enn_Spawner_C|SetReferent _asbp_enn_spawner (Variables|Default|GetReferent))
    (Variables|/Game/GD/Ennemis/BP_Enn_Spawner.BP_Enn_Spawner_C|SetFromBeginning _asbp_enn_spawner false)
    (Variables|/Game/GD/Ennemis/BP_Enn_Spawner.BP_Enn_Spawner_C|SetLibre _asbp_enn_spawner true)
    (Variables|/Game/GD/Ennemis/BP_Enn_Spawner.BP_Enn_Spawner_C|SetDesactiver _asbp_enn_spawner true)))

(fn ConstructionScript)