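; BP_Spawner is an enemy spawner actor that populates the area around itself with BP_EnnCac enemies once, one second after play begins.
; It loops over EnnemiNumber, spawning each enemy at a random reachable navmesh point within SpawnRadius, with collision adjustment that always allows the spawn.
; Each enemy gets Referent as its CrowdManager, and the collected list is then passed to Referent through AddEnnemis.
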(event Custom|SpawnEnnemies
  (for _index (range 0 (Variables|Default|GetEnnemiNumber))
    (bind _returnvalue (Game|SpawnActorfromClass "/Game/GD/Ennemis/Cac/BP_EnnCac.BP_EnnCac_C" (Math|Transform|MakeTransform (.RandomLocation (AI|Navigation|GetRandomReachablePointinRadius (Transformation|GetActorLocation) (Variables|Default|GetSpawnRadius) 0 0)) "0, 0, 0" "1.000000,1.000000,1.000000") "AdjustIfPossibleButAlwaysSpawn" "MultiplyWithRoot" 0 0))
    (Utilities|Array|Add (Variables|Default|GetSpawnedEnnemis) _returnvalue)
    (Variables|/Game/GD/Ennemis/Cac/BP_EnnCac.BP_EnnCac_C|SetCrowdManager _returnvalue (Variables|Default|GetReferent)))
  (Default|AddEnnemis (Variables|Default|GetReferent) (Variables|Default|GetSpawnedEnnemis)))

(event EventBeginPlay
  (Utilities|FlowControl|Delay 1.0)
  (CallFunction|SpawnEnnemies))

(event Collision|EventActorBeginOverlap
  (params (OtherActor :type Actor%20Object%20Reference)))

(event EventTick
  (params (DeltaSeconds :type Float%20%28single-precision%29)))

(fn ConstructionScript)