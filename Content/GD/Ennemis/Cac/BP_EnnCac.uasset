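; BP_EnnCac is an enemy character, apparently the melee ("Cac") variant, driven by AIC_EnnController.
; On BeginPlay it caches its controller, loads its health, damage, speed and water/electric stack and immunity stats from the Enn_Cac row of DT_StatEnnemis, then stores the BP_PP_Yass player.
; GoAttack_1 sets the player as move target and raises the ShouldAttack blackboard flag, handing the attack to the AI.
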(event Custom|SetMoveToTarget
  (params (NewTarget :type Actor%20Object%20Reference))
  (Variables|Default|SetMoveToTarget NewTarget))

(event Custom|GoAttack_1
  (Utilities|FlowControl|Sequence
    (:then_0
      (bind _asaic_enn_controller (Utilities|Casting|CastToAIC_EnnController (AI|GetAIController self)))
      (CallFunction|SetMovetoTarget (Variables|Default|GetPlayer))
      (AI|Components|Blackboard|SetValueasBool (AI|GetBlackboard _asaic_enn_controller) (Utilities|Name|MakeLiteralName "ShouldAttack") true))))

(event EventBeginPlay
  (bind _asaic_enn_controller (Utilities|Casting|CastToAIC_EnnController (AI|GetAIController self)))
  (Variables|Default|SetAIC _asaic_enn_controller)
  (bind _returnvalue (Utilities|GetDataTableRow "/Game/GD/Ennemis/Cac/DT_StatEnnemis.DT_StatEnnemis" "Enn_Cac")
    (:then
      (CallFunction|SetStats (.hpmax _returnvalue) (.damage _returnvalue) (.walkspeed _returnvalue) (.runspeed _returnvalue) (.watermaxstack _returnvalue) (.elecmaxstack _returnvalue) (.immunewater _returnvalue) (.immuneelec _returnvalue))
      (bind _asbp_pp_yass (Utilities|Casting|CastToBP_PP_Yass (Game|GetPlayerCharacter 0)))
      (Variables|Default|SetPlayer _asbp_pp_yass))))

(fn ConstructionScript
  (|CallParentFunction))