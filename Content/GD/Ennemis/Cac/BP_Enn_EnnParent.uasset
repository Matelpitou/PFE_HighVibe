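; Parent enemy Blueprint handling HP, damage, water/electric status stacks and death with loot and money.
; TakeDamage adds stacks unless immune, updates their display and can slow the enemy at full stacks.
; ProcEtat turns full stacks into bonus damage: electric stuns, while water briefly expands a sphere that chains procs through other water-stacked enemies.
; Death handling only covers BP_Enn_Cac, notifying its CrowdManager or destroying Crazy ones; hit and GoCrazy events are empty here.
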(event OnComponentBeginOverlap(WaterProcCollider)
  (params (OverlappedComponent :type Primitive%20Component%20Object%20Reference) (OtherActor :type Actor%20Object%20Reference) (OtherComp :type Primitive%20Component%20Object%20Reference) (OtherBodyIndex :type Integer) (bFromSweep :type Boolean) (SweepResult :type Hit%20Result%20Structure%20%28by%20ref%29))
  (bind _asbp_enn_enn_parent (Utilities|Casting|CastToBP_Enn_EnnParent OtherActor))
  (if (not (== _asbp_enn_enn_parent self))
    (CallFunction|ReceiveWaterProc _asbp_enn_enn_parent)))

(event Custom|TakeDamage
  (params (Damage :type Integer) (StackEau :type Integer) (StackElec :type Integer))
  (bind _systeco (Variables|Default|GetSystEco))
  (Variables|Default|SetAttacking false)
  (if (!= StackEau 0)
    (bind _elecproc (CallFunction|AddWater StackEau))
    (if _elecproc
      (Utilities|FlowControl|Sequence
        (:then_0
          _))
      (else
        (bind _above (CallFunction|ManageWaterSymbol))
        (if _above
          (CallFunction|GetSlowed)))))
  (if (!= StackElec 0)
    (bind _waterproc (CallFunction|AddElec StackElec))
    (if _waterproc
      (CallFunction|ManageElecSymbol)
      (else
        (bind _above_2 (CallFunction|ManageElecSymbol))
        (if _above_2
          (CallFunction|GetSlowed)))))
  (if (!= Damage 0)
    (bind _deadornot (CallFunction|LoseHP Damage))
    (if _deadornot
      (Game|SpawnActorfromClass "/Game/GD/Ennemis/Loot/BP_LootEnnemis.BP_LootEnnemis_C" (Transformation|GetActorTransform) "Undefined" "MultiplyWithRoot" 0 0)
      (Utilities|IsValid _systeco
        (:Is%20Valid
          (Default|GagnerArgent _systeco (Variables|Default|GetValeur)))
        (:Is%20Not%20Valid
          _))
      (CallFunction|Die)
      (else
        (CallFunction|PrepareSecondHit)
        (Utilities|FlowControl|DelayUntilNextTick)
        (CallFunction|HitAnimation)
        (if (Variables|Default|GetMoneyOnHit)
          (Default|GagnerArgent (Variables|Default|GetSystEco) (Variables|Default|GetValeur)))))))

(event Custom|GetSpeeded
  (Utilities|IsValid self
    (:Is%20Valid
      (Variables|/Script/Engine.CharacterMovementComponent|SetMaxWalkSpeed (Variables|Character|GetCharacterMovement) (Variables|Default|GetSpeedRun)))))

(event Custom|GetSlowed
  (Utilities|IsValid self
    (:Is%20Valid
      (Variables|/Script/Engine.CharacterMovementComponent|SetMaxWalkSpeed (Variables|Character|GetCharacterMovement) (Variables|Default|GetSpeedWalk)))))

(event Custom|HitAnimation)

(event Custom|Stunned
  (bind _elecsymbol (Variables|Default|GetElecSymbol))
  (Variables|Default|SetStunn true)
  (Utilities|IsValid _elecsymbol
    (:Is%20Valid
      (Development|SetHiddeninGame _elecsymbol false false))
    (:Is%20Not%20Valid
      _))
  (Utilities|FlowControl|Delay 2.0)
  (Utilities|IsValid self
    (:Is%20Valid
      (Utilities|IsValid _elecsymbol
        (:Is%20Valid
          (Development|SetHiddeninGame _elecsymbol true false)
          (Variables|Default|SetStunn false))))))

(event Custom|ForceWaterProc
  (bind _waterproccollider (Variables|Default|GetWaterProcCollider))
  (bind _watersymbol (Variables|Default|GetWaterSymbol))
  (Utilities|FlowControl|Sequence
    (:then_0
      (Components|Sphere|SetSphereRadius _waterproccollider (Variables|Default|GetWaterProcRadius) true)
      (Utilities|FlowControl|DelayUntilNextTick)
      (Utilities|IsValid _waterproccollider
        (:Is%20Valid
          (Components|Sphere|SetSphereRadius _waterproccollider 0.0 true))))
    (:then_1
      (Development|SetHiddeninGame _watersymbol false false)
      (Utilities|FlowControl|Delay 1.0)
      (Development|SetHiddeninGame _watersymbol true false))))

(event Custom|Recovery)

(event Custom|GoCrazy)

(event Custom|PrepareSecondHit)

(event Custom|ProcEtat
  (bind _systeco (Variables|Default|GetSystEco))
  (bind _waterisstacked (CallFunction|VerifStackWater))
  (if _waterisstacked
    (bind _elecisstacked (CallFunction|VerifStackElec))
    (if _elecisstacked
      (Utilities|FlowControl|Sequence
        (:then_0
          (Utilities|NewMacro :!label _label
            (:NewParam2
              (if (!= (stale Custom|TakeDamage Damage) 0)
                (bind _deadornot (CallFunction|LoseHP (stale Custom|TakeDamage Damage)))
                (if _deadornot
                  (Game|SpawnActorfromClass "/Game/GD/Ennemis/Loot/BP_LootEnnemis.BP_LootEnnemis_C" (Transformation|GetActorTransform) "Undefined" "MultiplyWithRoot" 0 0)
                  (Utilities|IsValid _systeco
                    (:Is%20Valid
                      (Default|GagnerArgent _systeco (Variables|Default|GetValeur)))
                    (:Is%20Not%20Valid
                      _))
                  (CallFunction|Die)
                  (else
                    (CallFunction|PrepareSecondHit)
                    (Utilities|FlowControl|DelayUntilNextTick)
                    (CallFunction|HitAnimation)
                    (if (Variables|Default|GetMoneyOnHit)
                      (Default|GagnerArgent (Variables|Default|GetSystEco) (Variables|Default|GetValeur)))))))))
        (:then_1
          (CallFunction|Stunned :!label _label_2)
          (Utilities|FlowControl|DelayUntilNextTick)
          (CallFunction|TakeDamage (* (Variables|Default|GetElecStack) (Variables|Default|GetDegatStack)))
          (Utilities|FlowControl|DelayUntilNextTick)
          (CallFunction|ClearStacks)))
      (else
        (goto _label)))
    (else
      (bind _elecisstacked_2 (CallFunction|VerifStackElec))
      (if _elecisstacked_2
        (goto _label_2)))))

(event EventBeginPlay
  (bind _asaic_enn_controller (Utilities|Casting|CastToAIC_EnnController (Pawn|GetController)))
  (Variables|Default|SetAIC _asaic_enn_controller)
  (Utilities|FlowControl|DelayUntilNextTick)
  (Utilities|Casting|CastToBP_PP_Yass (Game|GetPlayerCharacter 0))
  (Variables|Default|SetSystEco 0)
  (if (Variables|Default|GetCrazy)
    (CallFunction|GoCrazy)))

(fn ConstructionScript)

(fn LoseHP
  (params (DamageIncome :type Integer))
  (bind _output_get (Variables|Default|SetHP (Math|Integer|Clamp(Integer) (- (Variables|Default|GetHP) DamageIncome) 0 (Variables|Default|GetHPMax))))
  (return (== _output_get 0)))

(fn Die
  (bind _asbp_enn_cac (Utilities|Casting|CastToBP_Enn_Cac self))
  (Utilities|IsValid _asbp_enn_cac
    (:Is%20Valid
      (Default|Die (Variables|Default|GetAC_Element))
      (if (Variables|Default|GetCrazy)
        (Actor|DestroyActor)
        (else
          (Default|EnnemiDie (Variables|/Game/GD/Ennemis/Cac/BP_Enn_Cac.BP_Enn_Cac_C|GetCrowdManager _asbp_enn_cac) self)))
      (return))))

(fn GainHP
  (params (HealIncome :type Integer))
  (Variables|Default|SetHP (Math|Integer|Clamp(Integer) (+ HealIncome (Variables|Default|GetHP)) 0 (Variables|Default|GetHPMax)))
  (return))

(fn AddWater
  (params (IncomingWater :type Integer))
  (if (Variables|Default|GetImmuneWater)
    (LocalVariables|SetGoProc false)
    (else
      (Variables|Default|SetWaterStack (+ IncomingWater (Variables|Default|GetWaterStack)))
      (bind _elecisstacked (CallFunction|VerifStackElec))
      (LocalVariables|SetGoProc _elecisstacked)))
  (return (LocalVariables|GetGoProc)))

(fn AddElec
  (params (IncomingElec :type Integer))
  (if (Variables|Default|GetImmuneElec)
    (LocalVariables|SetGoProc false)
    (else
      (Variables|Default|SetElecStack (+ IncomingElec (Variables|Default|GetElecStack)))
      (bind _waterisstacked (CallFunction|VerifStackWater))
      (LocalVariables|SetGoProc _waterisstacked)))
  (return (LocalVariables|GetGoProc)))

(fn VerifStackWater
  (return (>= (Variables|Default|GetWaterStack) (Variables|Default|GetWaterMaxStack))))

(fn VerifStackElec
  (return (>= (Variables|Default|GetElecStack) (Variables|Default|GetElecMaxStack))))

(fn ProcWater)

(fn ManageWaterSymbol
  (Default|SetElec (Variables|Default|GetAC_Element) (Math|Integer|Clamp(Integer) (Variables|Default|GetElecStack) 0 (Variables|Default|GetElecMaxStack)) (Math|Integer|Clamp(Integer) (Variables|Default|GetWaterStack) 0 (Variables|Default|GetWaterMaxStack)))
  (bind _waterisstacked (CallFunction|VerifStackWater))
  (return _waterisstacked))

(fn ManageElecSymbol
  (bind _ac_element (Variables|Default|GetAC_Element))
  (Utilities|IsValid _ac_element
    (:Is%20Valid
      (Default|SetElec _ac_element (Math|Integer|Clamp(Integer) (Variables|Default|GetElecStack) 0 (Variables|Default|GetElecMaxStack)) (Math|Integer|Clamp(Integer) (Variables|Default|GetWaterStack) 0 (Variables|Default|GetWaterMaxStack)))
      (bind _elecisstacked (CallFunction|VerifStackElec))
      (return _elecisstacked))))

(fn ReceiveWaterProc
  (bind _waterstack (Variables|Default|GetWaterStack))
  (LocalVariables|SetNewLocalVar _waterstack)
  (if (> _waterstack 0)
    (CallFunction|ClearStacks)
    (CallFunction|ForceWaterProc)
    (CallFunction|TakeDamage (* (LocalVariables|GetNewLocalVar) (Variables|Default|GetDegatStack))))
  (return))

(fn SetStats
  (params (HPMax :type Integer) (Damage :type Integer) (WalkSpeed :type Float%20%28double-precision%29) (RunSpeed :type Float%20%28double-precision%29) (WaterMaxStack :type Integer) (ElecMaxStack :type Integer) (ImmuneWater :type Boolean) (ImmuneElec :type Boolean) (Valeur :type Integer))
  (bind _output_get (Variables|Default|SetHPMax HPMax))
  (Variables|Default|SetHP _output_get)
  (Variables|Default|SetDamage Damage)
  (Variables|Default|SetSpeedWalk WalkSpeed)
  (Variables|Default|SetSpeedRun RunSpeed)
  (Variables|Default|SetWaterMaxStack WaterMaxStack)
  (Variables|Default|SetElecMaxStack ElecMaxStack)
  (Variables|Default|SetImmuneWater ImmuneWater)
  (Variables|Default|SetImmuneElec ImmuneElec)
  (Variables|Default|SetValeur Valeur)
  (return))

(fn ClearStacks
  (Variables|Default|SetElecStack 0)
  (Variables|Default|SetWaterStack 0)
  (CallFunction|ManageElecSymbol)
  (CallFunction|GetSpeeded)
  (return))