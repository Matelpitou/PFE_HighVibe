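; Pyro melee enemy that fights the player with several hitbox attacks, a thrown physics beam (Poutre) and alternating waves of spawner reinforcements.
; BeginPlay loads stats from the enemy DataTable, randomizes its material, caches the player and binds to the force-nuke event.
; Events drive the AI through Blackboard keys for attack, stun, death and a one-time "KingKong" trigger at two-thirds HP.
; Death plays a timeline-driven dissolve on mesh and Niagara; the stun push-back chain is unconnected.
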(event Custom|SetMoveToTarget
  (params (NewTarget :type Actor%20Object%20Reference))
  ;[1 1 1] Set MoveToTarget
  (Variables|Default|SetMoveToTarget NewTarget))

(event Custom|SpawnHitBox
  (params (Enum :type Enum_PyroHitBox%20Enum :default "NewEnumerator0"))
  ;[1 1 1] Spawn HitBox
  (switch Utilities|FlowControl|Switch|SwitchonEnum_PyroHitBox Enum
    (:NewEnumerator0
      (Variables|Default|SetHitBoxClass "/Game/GD/Ennemis/Cac/Pyro/BP_HitBox_Front1.BP_HitBox_Front1_C"))
    (:NewEnumerator1
      (if (Variables|Hit|GetBackFist) :!label _label
        (Variables|Default|SetHitBoxClass "/Game/GD/Ennemis/Cac/Pyro/BP_HitBox_BackStab.BP_HitBox_BackStab_C")
        (else
          (Variables|Default|SetHitBoxClass "/Game/GD/Ennemis/Cac/Pyro/BP_HitBox_Front2.BP_HitBox_Front2_C"))))
    (:NewEnumerator2
      (goto _label))
    (:NewEnumerator3
      (Variables|Default|SetHitBoxClass "/Game/GD/Ennemis/Cac/Pyro/BP_HitBox_Booming.BP_HitBox_Booming_C"))
    (:NewEnumerator4
      (Variables|Default|SetHitBoxClass "/Game/GD/Ennemis/Cac/Pyro/BP_HitBox_ChargeHit.BP_HitBox_ChargeHit_C"))
    (:NewEnumerator5
      (Variables|Default|SetHitBoxClass "/Game/GD/Ennemis/Cac/Pyro/BP_HitBox_Poutre.BP_HitBox_Poutre_C"))
    (:NewEnumerator6
      (Variables|Default|SetHitBoxClass "/Game/GD/Ennemis/Cac/Pyro/BP_HitBox_JumpImpact.BP_HitBox_JumpImpact_C")))
  (Game|SpawnActorfromClass (Variables|Default|GetHitBoxClass) (Math|Transform|MakeTransform (Transformation|GetWorldLocation (Variables|Character|GetMesh)) (Transformation|GetActorRotation) "1.000000,1.000000,1.000000") "Undefined" "MultiplyWithRoot" 0 0))

(event Custom|FirstReco
  ;[1 1 1] Take Hit
  ;;[1 1 1] First Reco
  (AI|Components|Blackboard|SetValueasBool (Variables|/Script/AIModule.AIController|GetBlackboard (Variables|Default|GetAIC_0)) (Utilities|Name|MakeLiteralName "Stun") false))

(event Custom|Force%20nuke
  ;[1 1 1] Init
  (Variables|Default|SetGetNuke true)
  (CallFunction|TakeDamage 10000))

(event Custom|BOOM)

(event Custom|Spawn%20Ennemis
  (Utilities|FlowControl|FlipFlop
    (:A
      (for _array_element (Variables|Default|GetSpawners)
        (Default|ForceCombatParent _array_element)))
    (:B
      (for _array_element_2 (Variables|Default|GetSpawnersBis)
        (Default|ForceCombatParent _array_element_2)))))

(event Custom|StartKingKong)

(event Custom|LancerPoutre
  (bind _audiocomppyro (Variables|Default|GetAudioCompPyro))
  (bind _poutre (Variables|Default|GetPoutre))
  (bind _staticmesh1 (Variables|Default|GetStaticMesh1))
  (bind _player (Variables|Default|GetPlayer))
  (bind _returnvalue (Transformation|GetWorldLocation _staticmesh1))
  (bind _staticmesh (Variables|/Game/GD/Ennemis/Cac/Pyro/BP_Poutre.BP_Poutre_C|GetStaticMesh _poutre))
  (bind _mesh (Variables|/Script/Engine.Character|GetMesh _player))
  (bind _returnvalue_2 (Transformation|GetWorldLocation _mesh))
  (bind _returnvalue_3 (Math|Rotator|FindLookatRotation _returnvalue _returnvalue_2))
  (bind _returnvalue_4 (Game|SpawnActorfromClass "/Game/GD/Ennemis/Enn_Dist/BP_CircleProjectile.BP_CircleProjectile_C" (Math|Transform|MakeTransform _returnvalue_2 "0, 0, 0" "1.000000,1.000000,1.000000") "Undefined" "MultiplyWithRoot" 0 0))
  (Variables|/Game/GD/Ennemis/Cac/Pyro/BP_Poutre.BP_Poutre_C|SetTargetToDestroy (Variables|Default|GetPoutre) _returnvalue_4)
  (Utilities|FlowControl|Delay 0.2)
  (Transformation|SetWorldRotation _staticmesh _returnvalue_3 false false)
  (Physics|SetPhysicsLinearVelocity _staticmesh (* (Math|Vector|GetForwardVector _returnvalue_3) 3000) false "None")
  (Audio|Components|Audio|SetSound _audiocomppyro "/Game/GD/Ennemis/Son/s_throwpyrogadji.s_throwpyrogadji")
  (Audio|Components|Audio|Play _audiocomppyro 0.0))

(event Custom|SpawnPoutre
  (bind _staticmesh1 (Variables|Default|GetStaticMesh1))
  (bind _returnvalue (Transformation|GetWorldTransform _staticmesh1))
  (bind _returnvalue_2 (Game|SpawnActorfromClass "/Game/GD/Ennemis/Cac/Pyro/BP_Poutre.BP_Poutre_C" (Math|Transform|MakeTransform (.location _returnvalue) (.rotation _returnvalue) "1.000000,1.000000,1.000000") "Undefined" "MultiplyWithRoot" 0 0))
  (Variables|Default|SetPoutre _returnvalue_2))

(event Custom|GoAttack_1
  ;[1 1 1] Go attack
  (bind _asaic_enn_controller (Utilities|Casting|CastToAIC_EnnController (AI|GetAIController self)))
  (CallFunction|SetMovetoTarget (Variables|Default|GetPlayer))
  (AI|Components|Blackboard|SetValueasBool (AI|GetBlackboard _asaic_enn_controller) (Utilities|Name|MakeLiteralName "ShouldAttack") true))

(event EventBeginPlay
  ;[1 1 1] Init
  (bind _asaic_enn_controller (Utilities|Casting|CastToAIC_EnnController (AI|GetAIController self)))
  (Variables|Default|SetAIC_0 _asaic_enn_controller)
  (bind _returnvalue (Utilities|GetDataTableRow "/Game/GD/Ennemis/Cac/DT_Enn_StatEnnemis.DT_Enn_StatEnnemis" "Enn_Pyro")
    (:then
      (CallFunction|SetStats (.hpmax _returnvalue) (.damage _returnvalue) (.walkspeed _returnvalue) (.runspeed _returnvalue) (.watermaxstack _returnvalue) (.elecmaxstack _returnvalue) (.immunewater _returnvalue) (.immuneelec _returnvalue) (.valeur _returnvalue))
      (CallFunction|GetAColor)
      (bind _asbp_pp_yass (Utilities|Casting|CastToBP_PP_Yass (Game|GetPlayerCharacter 0)))
      (Utilities|FlowControl|Sequence
        (:then_0
          (Variables|Default|SetPlayer _asbp_pp_yass)
          (Variables|Default|SetSpawnLocation (Transformation|GetActorLocation))
          (if (Variables|Default|GetAfficherHP)
            (bind _aswb_hp_enn (Utilities|Casting|CastToWB_HP_Enn (UserInterface|GetUserWidgetObject (Variables|Default|GetWidget))))
            (Variables|Default|SetWB_HP _aswb_hp_enn)
            (Variables|/Game/GD/Ennemis/UI/WB_HP_Enn.WB_HP_Enn_C|SetOwner _aswb_hp_enn self)
            (else
              (Widget|SetVisibility (UserInterface|GetWidget (Variables|Default|GetWidget)) "Collapsed")))
          (EventDispatchers|BindEventtoForceNukeAllEnnemis (Variables|Default|GetNuker) (delegate Custom|Force%20nuke)))
        (:then_1
          (Utilities|FlowControl|Delay 0.2)
          (Variables|Default|SetMipMop (Variables|/Game/GD/PP/Yass/BP_PP_Yass.BP_PP_Yass_C|GetMipMop _asbp_pp_yass)))))))

(event EventHitAnimation
  ;[1 1 1] Take Hit
  (if (<= (Variables|Default|GetHP) (* (/ (Variables|Default|GetHPMax) 3) 2))
    (Variables|Default|SetNerf false)
    (Utilities|FlowControl|DoOnce false
      (:Completed
        (AI|Components|Blackboard|SetValueasBool (AI|GetBlackboard (Variables|Default|GetAIC_0)) (Utilities|Name|MakeLiteralName "KingKong") true)
        (Variables|Default|SetKingKongDone true)
        (Variables|Default|SetNerf true)))))

(event EventRecovery
  (bind _returnvalue (Utilities|Name|MakeLiteralName "ShouldAttack"))
  (bind _aic_0 (Variables|Default|GetAIC_0))
  (bind _blackboard (Variables|/Script/AIModule.AIController|GetBlackboard _aic_0))
  ;[1 1 1] Take Hit
  ;;[1 1 1] Recovery
  (Variables|Default|SetGettingHit false)
  (if (Variables|Default|GetStunn)
    (Utilities|FlowControl|Delay (Variables|Default|GetStunDuration))
    (Variables|Default|SetStunn false))
  (AI|Components|Blackboard|SetValueasBool _blackboard (Utilities|Name|MakeLiteralName "Stun") false)
  (if (Variables|Default|GetTempVarAttacking)
    (AI|Components|Blackboard|SetValueasBool _blackboard _returnvalue true)
    (Variables|Default|SetTempVarAttacking false)
    (else
      (AI|Components|Blackboard|SetValueasBool _blackboard _returnvalue false))))

(event EventPrepareSecondHit
  (bind _aic_0 (Variables|Default|GetAIC_0))
  (bind _returnvalue (AI|GetBlackboard _aic_0))
  ;[1 1 1] Multi Tap
  (if (ScalableFloat|GetValueasBool _returnvalue (Utilities|Name|MakeLiteralName "Stun"))
    (AI|Components|Blackboard|SetValueasBool _returnvalue (Utilities|Name|MakeLiteralName "Reset") true)))

(event EventGoCrazy
  ;[1 1 1] Go crazy
  (Variables|Default|SetCrazy true)
  (CallFunction|GoAttack1))

(event EventDieAnimation
  ;[1 1 1] Die
  (AI|Components|Blackboard|SetValueasBool (Variables|/Script/AIModule.AIController|GetBlackboard (Variables|Default|GetAIC_0)) (Utilities|Name|MakeLiteralName "Dead") true)
  (Utilities|FlowControl|Sequence
    (:then_0
      (Variables|Default|SetFalling true)
      (Utilities|FlowControl|Delay 1.5)
      (Variables|Default|SetDead true)
      (Utilities|FlowControl|Delay 0.5))
    (:then_1
      (Utilities|MacroShaderDestroy (Variables|Default|GetNiagara_0) (Variables|Character|GetMesh)
        (:NewParam
          (bind _newtrack_0 (Timeline|Timeline_1 PlayFromStart)
            (:Update
              (Rendering|Material|SetScalarParameterValueonMaterials (Variables|Character|GetMesh) "alpha" _newtrack_0)
              (Niagara|SetNiagaraVariable(Float) (Variables|Default|GetNiagara_0) "alpha" _newtrack_0))))))))

(fn ConstructionScript
  (|CallParentFunction))

(fn GetAColor
  (bind _material (Variables|Default|GetMaterial))
  (Rendering|Material|SetMaterial (Variables|Character|GetMesh) 0 (Utilities|Array|Get(acopy) _material (Math|Random|RandomIntegerinRange 0 (- (Utilities|Array|Length _material) 1))))
  (return))