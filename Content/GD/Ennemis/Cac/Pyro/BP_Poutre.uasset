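; BP_Poutre is a physics-driven beam from the Pyro enemy content that creates a damaging-style impact when it hits the BP_SolPyro floor.
; On BeginPlay, a reversed Timeline animates the dissolve alpha on dynamic materials and a matching Niagara effect, sharing texture and edge color.
; The first floor overlap freezes physics, plays sound, destroys TargetToDestroy, spawns BP_HitBox_JumpImpact and briefly activates the Impact effect.
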(event OnComponentBeginOverlap(StaticMesh)
  (params (OverlappedComponent :type Primitive%20Component%20Object%20Reference) (OtherActor :type Actor%20Object%20Reference) (OtherComp :type Primitive%20Component%20Object%20Reference) (OtherBodyIndex :type Integer) (bFromSweep :type Boolean) (SweepResult :type Hit%20Result%20Structure%20%28by%20ref%29))
  (bind _staticmesh (Variables|Default|GetStaticMesh))
  (bind _impact (Variables|Default|GetImpact))
  (Utilities|Casting|CastToBP_SolPyro OtherActor)
  (Utilities|FlowControl|DoOnce false
    (:Completed
      (Audio|PlaySoundatLocation "/Game/GD/Ennemis/Cac/Pyro/s_poutreimpact.s_poutreimpact" (Transformation|GetActorLocation) "0, 0, 0" 0.1 1.0 0.0 0 0 0 0)
      (Physics|SetPhysicsLinearVelocity _staticmesh "0, 0, 0" false "None")
      (Physics|SetSimulatePhysics _staticmesh false)
      (Actor|DestroyActor (Variables|Default|GetTargetToDestroy))
      (Game|SpawnActorfromClass "/Game/GD/Ennemis/Cac/Pyro/BP_HitBox_JumpImpact.BP_HitBox_JumpImpact_C" (Math|Transform|MakeTransform (Transformation|GetWorldLocation (Variables|Default|GetImpact)) "0, 0, 0" "1.000000,1.000000,1.000000") "Undefined" "MultiplyWithRoot" 0 0)
      (Components|Activation|Activate _impact false)
      (Utilities|FlowControl|Delay 1.5)
      (Components|Activation|Deactivate _impact))))

(event EventBeginPlay
  (bind _shader (Variables|Default|GetShader))
  (bind _staticmesh (Variables|Default|GetStaticMesh))
  (Rendering|Material|SetScalarParameterValueonMaterials _staticmesh "alpha" (Variables|Default|Getalpha))
  (Rendering|Material|SetVectorParameterValueonMaterials _staticmesh "edgecolor" (* (Math|Conversions|ToVector(LinearColor) (Variables|Default|Getedgecolor)) (Variables|Default|Getcolors_boost)))
  (Niagara|SetNiagaraVariable(Float) _shader "alpha" (Variables|Default|Getalpha))
  (Niagara|SetNiagaraVariable(LinearColor) _shader "edgecolor" (Variables|Default|Getedgecolor))
  (Niagara|SetTextureObject _shader "destroyagetexture" (Variables|Default|Gettexture))
  (for (_array_element _array_index) (Rendering|Material|GetMaterials _staticmesh)
    (bind _returnvalue (Rendering|Material|CreateDynamicMaterialInstance _staticmesh _array_index _array_element "None" :!class /Script/Engine.PrimitiveComponent))
    (Rendering|Material|SetTextureParameterValue _returnvalue "disolve" (Variables|Default|Gettexture))
    (bind _newtrack_0 (Timeline|Timeline ReverseFromEnd)
      (:Update
        (Rendering|Material|SetScalarParameterValueonMaterials (Variables|Default|GetStaticMesh) "alpha" _newtrack_0)
        (Niagara|SetNiagaraVariable(Float) (Variables|Default|GetShader) "alpha" _newtrack_0)))))

(fn ConstructionScript)