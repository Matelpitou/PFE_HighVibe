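; Melee enemy character that loads its stats from a data table, picks a random material and can dissolve in on spawn.
; Combat events drive its AI controller's blackboard for attack, stun, recovery and death, and spawn a forward hitbox.
; Hits trigger a traced, timeline-driven knockback and notify the crowd manager of surprise attacks.
; Death and optional reverse spawn share a dissolve macro syncing mesh materials with Niagara.
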(event Custom|SetMoveToTarget
  (params (NewTarget :type Actor%20Object%20Reference))
  ;[1 1 1] Set MoveToTarget
  (Variables|Default|SetMoveToTarget NewTarget))

(event Custom|SpawnHitBox
  ;[1 1 1] Spawn HitBox
  (bind _returnvalue (Game|SpawnActorfromClass "/Game/GD/Ennemis/Cac/BP_Enn_HitBox.BP_Enn_HitBox_C" (Math|Transform|MakeTransform (+ (Transformation|GetActorLocation) (* (Math|Vector|GetForwardVector (Transformation|GetActorRotation)) 100)) "0, 0, 0" "1.000000,1.000000,1.000000") "Undefined" "MultiplyWithRoot" 0 0))
  (Variables|/Game/GD/Ennemis/Cac/BP_Enn_HitBox.BP_Enn_HitBox_C|SetDamage _returnvalue (Variables|Default|GetDamage)))

(event Custom|FirstReco
  ;[1 1 1] Take Hit
  ;;[1 1 1] First Reco
  (AI|Components|Blackboard|SetValueasBool (Variables|/Script/AIModule.AIController|GetBlackboard (Variables|Default|GetAIC_0)) (Utilities|Name|MakeLiteralName "Stun") false))

(event Custom|Force%20nuke
  ;[1 1 1] Init
  (Variables|Default|SetGetNuke true)
  (CallFunction|TakeDamage 10000))

(event Custom|GoAttack_1
  ;[1 1 1] Go attack
  (Variables|Default|SetHasBeenAttacking true)
  (bind _asaic_enn_controller (Utilities|Casting|CastToAIC_EnnController (AI|GetAIController self)))
  (CallFunction|SetMovetoTarget (Variables|Default|GetPlayer))
  (AI|Components|Blackboard|SetValueasBool (AI|GetBlackboard _asaic_enn_controller) (Utilities|Name|MakeLiteralName "ShouldAttack") true))

(event EventBeginPlay
  ;[1 1 1] Init
  (bind _asaic_enn_controller (Utilities|Casting|CastToAIC_EnnController (AI|GetAIController self)))
  (Variables|Default|SetAIC_0 _asaic_enn_controller)
  (bind _returnvalue (Utilities|GetDataTableRow "/Game/GD/Ennemis/Cac/DT_Enn_StatEnnemis.DT_Enn_StatEnnemis" "Enn_Cac")
    (:then
      (CallFunction|SetStats (.hpmax _returnvalue) (.damage _returnvalue) (.walkspeed _returnvalue) (.runspeed _returnvalue) (.watermaxstack _returnvalue) (.elecmaxstack _returnvalue) (.immunewater _returnvalue) (.immuneelec _returnvalue) (.valeur _returnvalue))
      (CallFunction|GetAColor)
      (bind _asbp_pp_yass (Utilities|Casting|CastToBP_PP_Yass (Game|GetPlayerCharacter 0)))
      (Utilities|FlowControl|Sequence
        (:then_0
          (Variables|Default|SetPlayer _asbp_pp_yass)
          (Variables|Default|SetSpawnLocation (Transformation|GetActorLocation))
          (if (Variables|Default|GetAfficherHP)
            (bind _aswb_hp_enn (Utilities|Casting|CastToWB_HP_Enn (UserInterface|GetUserWidgetObject (Variables|Default|GetWidget))))
            (Variables|Default|SetWB_HP _aswb_hp_enn)
            (Variables|/Game/GD/Ennemis/UI/WB_HP_Enn.WB_HP_Enn_C|SetOwner _aswb_hp_enn self)
            (else
              (Widget|SetVisibility (UserInterface|GetWidget (Variables|Default|GetWidget)) "Collapsed")))
          (EventDispatchers|BindEventtoForceNukeAllEnnemis (Variables|Default|GetNuker) (delegate Custom|Force%20nuke))
          (if (Variables|Default|GetReverseSpawn)
            (Utilities|MacroShaderDestroy (Variables|Default|GetNiagara_0) (Variables|Character|GetMesh)
              (:NewParam
                (bind _newtrack_0 (Timeline|Timeline_2 ReverseFromEnd)
                  (:Update
                    (Rendering|Material|SetScalarParameterValueonMaterials (Variables|Character|GetMesh) "alpha" _newtrack_0)
                    (Niagara|SetNiagaraVariable(Float) (Variables|Default|GetNiagara_0) "alpha" _newtrack_0)))))))
        (:then_1
          (Utilities|FlowControl|Delay 0.2)
          (Variables|Default|SetMipMop (Variables|/Game/GD/PP/Yass/BP_PP_Yass.BP_PP_Yass_C|GetMipMop _asbp_pp_yass)))))))

(event EventHitAnimation
  (bind _aic_0 (Variables|Default|GetAIC_0))
  (bind _capsulecomponent (Variables|Default|GetCapsuleComponent))
  (bind _returnvalue (Transformation|GetWorldLocation _capsulecomponent))
  (bind _blackboard (Variables|/Script/AIModule.AIController|GetBlackboard _aic_0))
  (bind (_x _y _z) (Math|Vector|BreakVector _returnvalue))
  (bind _returnvalue_2 (+ _z 5e+01))
  (bind _returnvalue_3 (Math|Vector|MakeVector _x _y _returnvalue_2))
  ;[1 1 1] Take Hit
  (Utilities|FlowControl|Gate false :!label _label
    (:Exit
      (Utilities|FlowControl|Sequence
        (:then_0
          (goto _label Close))
        (:then_1
          (Variables|Default|SetGettingHit false)
          (Utilities|FlowControl|DelayUntilNextTick)
          (if (ScalableFloat|GetValueasBool _blackboard (Utilities|Name|MakeLiteralName "ShouldAttack"))
            (Variables|Default|SetTempVarAttacking true))
          (Variables|Default|SetAttacking false)
          (Variables|Default|SetGettingHit true)
          (AI|Components|Blackboard|SetValueasBool _blackboard (Utilities|Name|MakeLiteralName "ShouldAttack") false)
          (AI|Components|Blackboard|SetValueasBool _blackboard (Utilities|Name|MakeLiteralName "Stun") true)
          (Utilities|FlowControl|Delay 0.2)
          (goto _label Open))
        (:then_2
          ;;[1 1 1] Push back
          (if (not (Variables|Default|GetStunn))
            (Variables|Default|SetSavedTransform (Transformation|GetActorTransform))
            (bind _returnvalue_4 (Collision|LineTraceByChannel _returnvalue_3 (- _returnvalue_3 (* (Math|Vector|GetForwardVector (Transformation|GetWorldRotation _capsulecomponent)) 1.2e+02)) "TraceTypeQuery1" true 0 "None"))
            (if (not _returnvalue_4)
              (bind _newtrack_0 (Timeline|Timeline_0 PlayFromStart)
                (:Update
                  (Transformation|SetActorLocation (Math|Vector|Lerp(Vector) (.location (Variables|Default|GetSavedTransform)) (+ (.location (Variables|Default|GetSavedTransform)) (* (Math|Vector|GetForwardVector (.rotation (Variables|Default|GetSavedTransform))) -7e+01)) _newtrack_0) false false))))))
        (:then_3
          (if (not (Variables|Default|GetHasBeenAttacking))
            (Default|EnnemiDie (Variables|Default|GetCrowdManager) self true)))))))

(event EventRecovery
  (bind _returnvalue (Utilities|Name|MakeLiteralName "ShouldAttack"))
  (bind _aic_0 (Variables|Default|GetAIC_0))
  (bind _blackboard (Variables|/Script/AIModule.AIController|GetBlackboard _aic_0))
  ;[1 1 1] Take Hit
  ;;[1 1 1] Recovery
  (Variables|Default|SetGettingHit false)
  (if (Variables|Default|GetStunn)
    (Utilities|FlowControl|Delay (Variables|Default|GetStunDuration))
    (Variables|Default|SetStunn false))
  (AI|Components|Blackboard|SetValueasBool _blackboard (Utilities|Name|MakeLiteralName "Stun") false)
  (if (Variables|Default|GetTempVarAttacking)
    (AI|Components|Blackboard|SetValueasBool _blackboard _returnvalue true)
    (Variables|Default|SetTempVarAttacking false)
    (else
      (AI|Components|Blackboard|SetValueasBool _blackboard _returnvalue false))))

(event EventPrepareSecondHit
  (bind _aic_0 (Variables|Default|GetAIC_0))
  (bind _returnvalue (AI|GetBlackboard _aic_0))
  ;[1 1 1] Multi Tap
  (if (ScalableFloat|GetValueasBool _returnvalue (Utilities|Name|MakeLiteralName "Stun"))
    (AI|Components|Blackboard|SetValueasBool _returnvalue (Utilities|Name|MakeLiteralName "Reset") true)))

(event EventGoCrazy
  ;[1 1 1] Go crazy
  (Variables|Default|SetCrazy true)
  (CallFunction|GoAttack1))

(event EventDieAnimation
  ;[1 1 1] Die
  (AI|Components|Blackboard|SetValueasBool (Variables|/Script/AIModule.AIController|GetBlackboard (Variables|Default|GetAIC_0)) (Utilities|Name|MakeLiteralName "Dead") true)
  (Utilities|FlowControl|Sequence
    (:then_0
      (Variables|Default|SetFalling true)
      (Utilities|FlowControl|Delay 1.5)
      (Variables|Default|SetDead true)
      (Utilities|FlowControl|Delay 0.5))
    (:then_1
      (Utilities|MacroShaderDestroy (Variables|Default|GetNiagara_0) (Variables|Character|GetMesh)
        (:NewParam
          (bind _newtrack_0 (Timeline|Timeline_1 PlayFromStart)
            (:Update
              (Rendering|Material|SetScalarParameterValueonMaterials (Variables|Character|GetMesh) "alpha" _newtrack_0)
              (Niagara|SetNiagaraVariable(Float) (Variables|Default|GetNiagara_0) "alpha" _newtrack_0))))))))

(fn ConstructionScript
  (|CallParentFunction))

(fn GetAColor
  (bind _material (Variables|Default|GetMaterial))
  (Rendering|Material|SetMaterial (Variables|Character|GetMesh) 0 (Utilities|Array|Get(acopy) _material (Math|Random|RandomIntegerinRange 0 (- (Utilities|Array|Length _material) 1))))
  (return))