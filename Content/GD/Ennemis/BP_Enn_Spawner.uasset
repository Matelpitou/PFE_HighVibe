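; Enemy spawner that places a group of BP_Enn_Cac at random reachable points within a radius.
; Enemies spawn either at BeginPlay (FromBeginning) or upon activation, which fires once through ForceSpawn or BP_PP_Yass entering the Box unless Desactiver is set.
; On activation, Libre enemies turn Crazy and attack independently, while others are handed as a batch to the Referent crowd manager.
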(event OnComponentBeginOverlap(Box)
  (params (OverlappedComponent :type Primitive%20Component%20Object%20Reference) (OtherActor :type Actor%20Object%20Reference) (OtherComp :type Primitive%20Component%20Object%20Reference) (OtherBodyIndex :type Integer) (bFromSweep :type Boolean) (SweepResult :type Hit%20Result%20Structure%20%28by%20ref%29))
  (bind _tempennspawned (Variables|Default|GetTempEnnSpawned))
  (bind _libre (Variables|Default|GetLibre))
  (if (not (Variables|Default|GetDesactiver))
    (Utilities|Casting|CastToBP_PP_Yass OtherActor)
    (Utilities|FlowControl|DoOnce false
      (:Completed
        (if (Variables|Default|GetFromBeginning)
          (for _array_element _tempennspawned
            (if _libre
              (Variables|/Game/GD/Ennemis/Cac/BP_Enn_EnnParent.BP_Enn_EnnParent_C|SetCrazy _array_element true)
              (Default|GoAttack1 _array_element)))
          (if (not _libre)
            (Default|AddEnnemis (Variables|Default|GetReferent) _tempennspawned))
          (elif (Variables|Default|GetLibre)
            (for _index (range 0 (Variables|Default|GetEnnemiNumber))
              (bind _returnvalue (Game|SpawnActorfromClass "/Game/GD/Ennemis/Cac/BP_Enn_Cac.BP_Enn_Cac_C" (Math|Transform|MakeTransform (.RandomLocation (AI|Navigation|GetRandomReachablePointinRadius (Transformation|GetActorLocation) (Variables|Default|GetSpawnRadius) 0 0)) "0, 0, 0" "1.000000,1.000000,1.000000") "AdjustIfPossibleButAlwaysSpawn" "MultiplyWithRoot" 0 0))
              (Variables|/Game/GD/Ennemis/Cac/BP_Enn_EnnParent.BP_Enn_EnnParent_C|SetCrazy _returnvalue true)
              (Variables|/Game/GD/Ennemis/Cac/BP_Enn_EnnParent.BP_Enn_EnnParent_C|SetSystEco _returnvalue (Variables|Default|GetSystEco))
              (Default|GoAttack1 _returnvalue))
            (else
              (for _index_2 (range 0 (Variables|Default|GetEnnemiNumber))
                (bind _returnvalue_2 (Game|SpawnActorfromClass "/Game/GD/Ennemis/Cac/BP_Enn_Cac.BP_Enn_Cac_C" (Math|Transform|MakeTransform (.RandomLocation (AI|Navigation|GetRandomReachablePointinRadius (Transformation|GetActorLocation) (Variables|Default|GetSpawnRadius) 0 0)) "0, 0, 0" "1.000000,1.000000,1.000000") "AdjustIfPossibleButAlwaysSpawn" "MultiplyWithRoot" 0 0))
                (Utilities|Array|Add (Variables|Default|GetSpawnedEnnemis) _returnvalue_2)
                (Variables|/Game/GD/Ennemis/Cac/BP_Enn_Cac.BP_Enn_Cac_C|SetCrowdManager _returnvalue_2 (Variables|Default|GetReferent))
                (Variables|/Game/GD/Ennemis/Cac/BP_Enn_EnnParent.BP_Enn_EnnParent_C|SetSystEco _returnvalue_2 (Variables|Default|GetSystEco)))
              (Default|AddEnnemis (Variables|Default|GetReferent) (Variables|Default|GetSpawnedEnnemis)))))))))

(event Custom|ForceSpawn
  (bind _tempennspawned (Variables|Default|GetTempEnnSpawned))
  (bind _libre (Variables|Default|GetLibre))
  (Utilities|FlowControl|DoOnce false
    (:Completed
      (if (Variables|Default|GetFromBeginning)
        (for _array_element _tempennspawned
          (if _libre
            (Variables|/Game/GD/Ennemis/Cac/BP_Enn_EnnParent.BP_Enn_EnnParent_C|SetCrazy _array_element true)
            (Default|GoAttack1 _array_element)))
        (if (not _libre)
          (Default|AddEnnemis (Variables|Default|GetReferent) _tempennspawned))
        (elif (Variables|Default|GetLibre)
          (for _index (range 0 (Variables|Default|GetEnnemiNumber))
            (bind _returnvalue (Game|SpawnActorfromClass "/Game/GD/Ennemis/Cac/BP_Enn_Cac.BP_Enn_Cac_C" (Math|Transform|MakeTransform (.RandomLocation (AI|Navigation|GetRandomReachablePointinRadius (Transformation|GetActorLocation) (Variables|Default|GetSpawnRadius) 0 0)) "0, 0, 0" "1.000000,1.000000,1.000000") "AdjustIfPossibleButAlwaysSpawn" "MultiplyWithRoot" 0 0))
            (Variables|/Game/GD/Ennemis/Cac/BP_Enn_EnnParent.BP_Enn_EnnParent_C|SetCrazy _returnvalue true)
            (Variables|/Game/GD/Ennemis/Cac/BP_Enn_EnnParent.BP_Enn_EnnParent_C|SetSystEco _returnvalue (Variables|Default|GetSystEco))
            (Default|GoAttack1 _returnvalue))
          (else
            (for _index_2 (range 0 (Variables|Default|GetEnnemiNumber))
              (bind _returnvalue_2 (Game|SpawnActorfromClass "/Game/GD/Ennemis/Cac/BP_Enn_Cac.BP_Enn_Cac_C" (Math|Transform|MakeTransform (.RandomLocation (AI|Navigation|GetRandomReachablePointinRadius (Transformation|GetActorLocation) (Variables|Default|GetSpawnRadius) 0 0)) "0, 0, 0" "1.000000,1.000000,1.000000") "AdjustIfPossibleButAlwaysSpawn" "MultiplyWithRoot" 0 0))
              (Utilities|Array|Add (Variables|Default|GetSpawnedEnnemis) _returnvalue_2)
              (Variables|/Game/GD/Ennemis/Cac/BP_Enn_Cac.BP_Enn_Cac_C|SetCrowdManager _returnvalue_2 (Variables|Default|GetReferent))
              (Variables|/Game/GD/Ennemis/Cac/BP_Enn_EnnParent.BP_Enn_EnnParent_C|SetSystEco _returnvalue_2 (Variables|Default|GetSystEco)))
            (Default|AddEnnemis (Variables|Default|GetReferent) (Variables|Default|GetSpawnedEnnemis))))))))

(event EventBeginPlay
  (if (Variables|Default|GetFromBeginning)
    (for _index (range 0 (Variables|Default|GetEnnemiNumber))
      (bind _returnvalue (Game|SpawnActorfromClass "/Game/GD/Ennemis/Cac/BP_Enn_Cac.BP_Enn_Cac_C" (Math|Transform|MakeTransform (.RandomLocation (AI|Navigation|GetRandomReachablePointinRadius (Transformation|GetActorLocation) (Variables|Default|GetSpawnRadius) 0 0)) "0, 0, 0" "1.000000,1.000000,1.000000") "AdjustIfPossibleButAlwaysSpawn" "MultiplyWithRoot" 0 0))
      (Utilities|Array|Add (Variables|Default|GetTempEnnSpawned) _returnvalue)
      (Variables|/Game/GD/Ennemis/Cac/BP_Enn_EnnParent.BP_Enn_EnnParent_C|SetSystEco _returnvalue (Variables|Default|GetSystEco))
      (Variables|/Game/GD/Ennemis/Cac/BP_Enn_Cac.BP_Enn_Cac_C|SetCrowdManager _returnvalue (Variables|Default|GetReferent)))))

(fn ConstructionScript)