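; Combat arena that locks the player in behind two walls until the fight is over, with optional dialogue before and after.
; On first box overlap by BP_PP_Yass, it shows the walls, waits a delay, then force-spawns from its spawners.
; Enemies register through AddEnnemi, which starts a looping timer polling their validity.
; Once none remain valid, the walls drop and post-battle dialogue spawns via a BP_DialogueTrigger at the player.
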(event OnComponentBeginOverlap(Box)
  (params (OverlappedComponent :type Primitive%20Component%20Object%20Reference) (OtherActor :type Actor%20Object%20Reference) (OtherComp :type Primitive%20Component%20Object%20Reference) (OtherBodyIndex :type Integer) (bFromSweep :type Boolean) (SweepResult :type Hit%20Result%20Structure%20%28by%20ref%29))
  ;[1 1 1] Begin overlap
  (Utilities|Casting|CastToBP_PP_Yass OtherActor)
  (Utilities|FlowControl|DoOnce false
    (:Completed
      (CallFunction|PreSpawnEvent))))

(event Custom|AddEnnemi
  (params (NewEnnemi :type BP%20Enn%20Enn%20Parent%20Object%20Reference))
  ;[1 1 1] Add ennemi
  (Utilities|FlowControl|Sequence
    (:then_0
      ;[1 1 1] Set timer check finish
      (Utilities|FlowControl|DoOnce false
        (:Completed
          (bind _returnvalue (Utilities|Time|SetTimerbyEvent (delegate Custom|CheckFinish) 5.0 true))
          (Variables|Default|SetTimerEndCombat _returnvalue))))
    (:then_1
      (Utilities|Array|Add (Variables|Default|GetEnnemiList) NewEnnemi))))

(event Custom|CheckFinish
  (bind _ennemilist (Variables|Default|GetEnnemiList))
  (bind _textapresbataille (Variables|Default|GetTextApresBataille))
  ;[1 1 1] Check finish
  (Variables|Default|SetContinue false)
  (for _index (range 0 (- (Utilities|Array|Length _ennemilist) 0))
    (if (Utilities|IsValid (Utilities|Array|Get(acopy) _ennemilist _index))
      (Variables|Default|SetContinue true)))
  ;[1 1 1] End of event, walls off
  (if (not (Variables|Default|GetContinue))
    (Utilities|Time|ClearandInvalidateTimerbyHandle (Variables|Default|GetTimerEndCombat))
    (CallFunction|WallsOff)
    (if (> (Utilities|Array|Length _textapresbataille) 0)
      (CallFunction|SpawnDialogue _textapresbataille (Variables|Default|GetQuiParleApresBataille)))))

(event Custom|SpawnWalls
  (bind _staticmesh1 (Variables|Default|GetStaticMesh1))
  (bind _staticmesh (Variables|Default|GetStaticMesh))
  ;[1 1 1] Spawn Walls
  (Development|SetHiddeninGame _staticmesh false false)
  (Development|SetHiddeninGame _staticmesh1 false false)
  (Collision|SetCollisionEnabled _staticmesh "QueryAndPhysics")
  (Collision|SetCollisionEnabled _staticmesh1 "QueryAndPhysics"))

(event Custom|PreSpawnEvent
  (bind _textavantbataille (Variables|Default|GetTextAvantBataille))
  ;[1 1 1] Pre_Spawn Event
  (if (> (Utilities|Array|Length _textavantbataille) 0)
    (CallFunction|SpawnDialogue _textavantbataille (Variables|Default|GetQuiParleAvantBataille)))
  (CallFunction|SpawnWalls)
  (Utilities|FlowControl|Delay (Variables|Default|GetDelayPreSpawn))
  (for _array_element (Variables|Default|GetSpawners)
    (Default|ForceSpawnParent _array_element)))

(event Custom|SpawnDialogue
  (params (Text :type Array%20of%20Texts) (QuiParle :type Array%20of%20Booleans))
  ;[1 1 1] Dialogue pre_spawn
  (bind _asbp_pp_yass (Utilities|Casting|CastToBP_PP_Yass (Game|GetPlayerCharacter 0)))
  (Game|SpawnActorfromClass "/Game/GD/Dialogues/BP_DialogueTrigger.BP_DialogueTrigger_C" (Transformation|GetActorTransform _asbp_pp_yass) "Undefined" "MultiplyWithRoot" 0 Text QuiParle 0))

(event EventBeginPlay
  ;[1 1 1] Set Walls off start of the game
  (CallFunction|WallsOff))

(fn ConstructionScript)

(fn WallsOff
  (bind _staticmesh1 (Variables|Default|GetStaticMesh1))
  (bind _staticmesh (Variables|Default|GetStaticMesh))
  (Development|SetHiddeninGame _staticmesh true false)
  (Development|SetHiddeninGame _staticmesh1 true false)
  (Collision|SetCollisionEnabled _staticmesh "NoCollision")
  (Collision|SetCollisionEnabled _staticmesh1 "NoCollision"))