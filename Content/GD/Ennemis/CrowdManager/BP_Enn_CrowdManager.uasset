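; Crowd manager that positions enemies around the player and caps how many attack at once.
; A looping EQS query around the player repositions a pool of target points spawned from its first result.
; New enemies claim free points from the array's end; while attack slots remain, one, preferably random among the last six points, is sent to attack.
; The first occupied point's enemy fills the vacancy, and deaths trigger new attack checks.
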(event Custom|AddEnnemis
  (params (EnnemisInput :type Array%20of%20BP%20Enn%20Cac%20Object%20References))
  (bind _ennemilist (Variables|Default|GetEnnemiList))
  (bind _alltargetpoints (Variables|Default|GetAllTargetPoints))
  (bind _returnvalue (Utilities|Array|Length _alltargetpoints))
  (bind _returnvalue_2 (- _returnvalue 1))
  ;[1 1 1] Add ennemis à la liste
  (for _index (range 0 (- (Utilities|Array|Length EnnemisInput) 1))
    (bind _returnvalue_3 (Utilities|Array|Add _ennemilist (Utilities|Array|Get(acopy) EnnemisInput _index)))
    ;[1 1 1] Donner Emplacement
    (bind _index_2 (Utilities|FlowControl|ForLoopwithBreak 0 _returnvalue_2 :!label _label)
      (:LoopBody
        (if (not (Variables|/Game/GD/Ennemis/CrowdManager/BP_Enn_TargetPoint.BP_Enn_TargetPoint_C|GetOccupe (Utilities|Array|Get(acopy) _alltargetpoints (- _returnvalue_2 _index_2))))
          (Variables|/Game/GD/Ennemis/CrowdManager/BP_Enn_TargetPoint.BP_Enn_TargetPoint_C|SetOccupe (Utilities|Array|Get(acopy) _alltargetpoints (- _returnvalue_2 _index_2)) true)
          (Variables|/Game/GD/Ennemis/CrowdManager/BP_Enn_TargetPoint.BP_Enn_TargetPoint_C|SetEnnemiHere (Utilities|Array|Get(acopy) _alltargetpoints (- _returnvalue_2 _index_2)) (Utilities|Array|Get(acopy) _ennemilist _returnvalue_3))
          (Default|SetMovetoTarget (Utilities|Array|Get(acopy) _ennemilist _returnvalue_3) (Utilities|Array|Get(acopy) _alltargetpoints (- _returnvalue_2 _index_2)))
          (goto _label Break)))))
  (CallFunction|AgroEnnemis))

(event Custom|RunEqsEvent
  (bind _returnvalue (AI|EQS|RunEQSQuery "/Game/GD/Ennemis/CrowdManager/EQS_CrowdManager.EQS_CrowdManager" (Variables|Default|GetPlayer) "AllMatching"))
  (EventDispatchers|BindEventtoOnQueryFinishedEvent _returnvalue (delegate Custom|MiseAJourEQS)))

(event Custom|MiseAJourEQS
  (params (QueryInstance :type Env%20Query%20Instance%20Blueprint%20Wrapper%20Object%20Reference) (QueryStatus :type EEnvQueryStatus%20Enum :default "Processing"))
  (bind _resultlocations (AI|EQS|GetQueryResultsasLocations QueryInstance))
  (Utilities|FlowControl|Sequence
    (:then_0
      (Utilities|FlowControl|DoOnce false
        (:Completed
          (CallFunction|SpawnTargetPoint _resultlocations))))
    (:then_1
      (Utilities|FlowControl|DelayUntilNextTick)
      (CallFunction|SetTargetPosition _resultlocations))))

(event Custom|RemoveEnnemi
  (bind _alltargetpoints (Variables|Default|GetAllTargetPoints))
  ;[1 1 1] Remove ennemi
  (bind _output_get (Variables|Default|SetTempVarTargetPoint (Utilities|Array|Get(acopy) _alltargetpoints (- (Utilities|Array|LastIndex _alltargetpoints) (Math|Random|RandomIntegerinRange 0 5)))))
  (Utilities|IsValid (Variables|/Game/GD/Ennemis/CrowdManager/BP_Enn_TargetPoint.BP_Enn_TargetPoint_C|GetEnnemiHere _output_get)
    (:Is%20Valid
      (CallFunction|SendtoPoint _output_get))
    (:Is%20Not%20Valid
      (bind _array_element (Utilities|Array|ForEachLoopwithBreak _alltargetpoints :!label _label)
        (:LoopBody
          (Utilities|IsValid (Variables|/Game/GD/Ennemis/CrowdManager/BP_Enn_TargetPoint.BP_Enn_TargetPoint_C|GetEnnemiHere _array_element)
            (:Is%20Valid
              (Utilities|FlowControl|Sequence
                (:then_0
                  (goto _label Break))
                (:then_1
                  (CallFunction|SendtoPoint _array_element))))))))))

(event Custom|NewOrder
  (bind _temptargetpoint (Variables|Default|GetTempTargetPoint))
  (bind _alltargetpoints (Variables|Default|GetAllTargetPoints))
  ;[1 1 1] Re ranger les ennemis et les emplacements
  (bind _index (Utilities|FlowControl|ForLoopwithBreak 0 (- (Utilities|Array|Length _alltargetpoints) 1) :!label _label)
    (:LoopBody
      (if (Variables|/Game/GD/Ennemis/CrowdManager/BP_Enn_TargetPoint.BP_Enn_TargetPoint_C|GetOccupe (Utilities|Array|Get(acopy) _alltargetpoints _index))
        (Variables|/Game/GD/Ennemis/CrowdManager/BP_Enn_TargetPoint.BP_Enn_TargetPoint_C|SetOccupe (Utilities|Array|Get(acopy) _alltargetpoints _index) false)
        (Utilities|IsValid (Variables|/Game/GD/Ennemis/CrowdManager/BP_Enn_TargetPoint.BP_Enn_TargetPoint_C|GetEnnemiHere (Utilities|Array|Get(acopy) _alltargetpoints _index))
          (:Is%20Valid
            (Variables|/Game/GD/Ennemis/CrowdManager/BP_Enn_TargetPoint.BP_Enn_TargetPoint_C|SetEnnemiHere _temptargetpoint (Variables|/Game/GD/Ennemis/CrowdManager/BP_Enn_TargetPoint.BP_Enn_TargetPoint_C|GetEnnemiHere (Utilities|Array|Get(acopy) _alltargetpoints _index))))
          (:Is%20Not%20Valid
            _))
        (Utilities|IsValid (Variables|/Game/GD/Ennemis/CrowdManager/BP_Enn_TargetPoint.BP_Enn_TargetPoint_C|GetEnnemiHere (Utilities|Array|Get(acopy) _alltargetpoints _index))
          (:Is%20Valid
            (Default|SetMovetoTarget (Variables|/Game/GD/Ennemis/CrowdManager/BP_Enn_TargetPoint.BP_Enn_TargetPoint_C|GetEnnemiHere (Utilities|Array|Get(acopy) _alltargetpoints _index)) _temptargetpoint))
          (:Is%20Not%20Valid
            _))
        (Variables|/Game/GD/Ennemis/CrowdManager/BP_Enn_TargetPoint.BP_Enn_TargetPoint_C|SetOccupe _temptargetpoint true)
        (Variables|/Game/GD/Ennemis/CrowdManager/BP_Enn_TargetPoint.BP_Enn_TargetPoint_C|SetEnnemiHere (Utilities|Array|Get(acopy) _alltargetpoints _index) 0)
        (goto _label Break)))
    (:Completed
      (Utilities|FlowControl|DelayUntilNextTick)
      (CallFunction|AgroEnnemis))))

(event Custom|EnnemiDie
  (params (QuiMeurt :type BP%20Enn%20Enn%20Parent%20Object%20Reference))
  ;[1 1 1] Mort d'un ennemi
  (Utilities|IsValid QuiMeurt
    (:Is%20Valid
      (bind _asaic_enn_controller (Utilities|Casting|CastToAIC_EnnController (AI|GetAIController QuiMeurt)))
      (if (ScalableFloat|GetValueasBool (Variables|/Script/AIModule.AIController|GetBlackboard _asaic_enn_controller) (Utilities|Name|MakeLiteralName "ShouldAttack"))
        (Actor|DestroyActor QuiMeurt :!label _label)
        (Variables|Default|SetNbCac (- (Variables|Default|GetNbCac) 1))
        (elif (Variables|/Game/GD/Ennemis/Cac/BP_Enn_EnnParent.BP_Enn_EnnParent_C|GetTempVarAttacking QuiMeurt)
          (goto _label)
          (else
            (Actor|DestroyActor QuiMeurt))))
      (CallFunction|AgroEnnemis))))

(event Custom|AgroEnnemis
  ;[1 1 1] Agro Ennemis
  (if (<= (Variables|Default|GetNbCac) (Variables|Default|GetLimitCac))
    (Variables|Default|SetNbCac (+ (Variables|Default|GetNbCac) 1))
    (CallFunction|RemoveEnnemi)))

(event EventBeginPlay
  (bind _asbp_pp_yass (Utilities|Casting|CastToBP_PP_Yass (Game|GetPlayerCharacter 0)))
  (Variables|Default|SetPlayer _asbp_pp_yass)
  (Utilities|Time|SetTimerbyEvent (delegate Custom|RunEqsEvent) 0.5 true))

(fn ConstructionScript)

(fn SpawnTargetPoint
  (params (NewParam :type Array%20of%20Vectors))
  (for _index (range 0 (- (Utilities|Array|Length NewParam) 1))
    (if (not (>= _index (Variables|Default|GetLimiteDeProximite)))
      (bind _returnvalue (Game|SpawnActorfromClass "/Game/GD/Ennemis/CrowdManager/BP_Enn_TargetPoint.BP_Enn_TargetPoint_C" (Math|Transform|MakeTransform (Utilities|Array|Get(acopy) NewParam _index) "0, 0, 0" "1.000000,1.000000,1.000000") "AdjustIfPossibleButAlwaysSpawn" "MultiplyWithRoot" 0 0))
      (bind _returnvalue_2 (Utilities|Array|Add (Variables|Default|GetAllTargetPoints) _returnvalue))
      (Rendering|Components|TextRender|SetText (Variables|/Game/GD/Ennemis/CrowdManager/BP_Enn_TargetPoint.BP_Enn_TargetPoint_C|GetTextRender _returnvalue) (Utilities|Text|ToText(Integer) _returnvalue_2)))))

(fn SetTargetPosition
  (params (NewParam :type Array%20of%20Vectors))
  (for _index (range 0 (- (Utilities|Array|Length NewParam) 1))
    (Utilities|IsValid (Utilities|Array|Get(acopy) (Variables|Default|GetAllTargetPoints) _index)
      (:Is%20Valid
        (Transformation|SetActorLocation (Utilities|Array|Get(acopy) (Variables|Default|GetAllTargetPoints) _index) (Utilities|Array|Get(acopy) NewParam _index) false false)))))

(fn SendtoPoint
  (params (NewParam :type BP%20Enn%20Target%20Point%20Object%20Reference))
  (bind _output_get (Variables|Default|SetTempTargetPoint NewParam))
  (Default|GoAttack1 (Variables|/Game/GD/Ennemis/CrowdManager/BP_Enn_TargetPoint.BP_Enn_TargetPoint_C|GetEnnemiHere _output_get))
  (Utilities|Array|RemoveItem (Variables|Default|GetEnnemiList) (Variables|/Game/GD/Ennemis/CrowdManager/BP_Enn_TargetPoint.BP_Enn_TargetPoint_C|GetEnnemiHere _output_get))
  (Variables|/Game/GD/Ennemis/CrowdManager/BP_Enn_TargetPoint.BP_Enn_TargetPoint_C|SetOccupe _output_get false)
  (Variables|/Game/GD/Ennemis/CrowdManager/BP_Enn_TargetPoint.BP_Enn_TargetPoint_C|SetEnnemiHere _output_get 0)
  (CallFunction|NewOrder)
  (return))