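; BP_SpawnerParent is a base Blueprint for enemy spawners with a door that swings open.
; OpenDoor caches the RootDoor world rotation, then a timeline lerps its yaw by AnglePorte while keeping roll and pitch.
; When the timeline finishes it calls GoBackToSpawn, which is empty here, as is ForceCombatParent, apparently as hooks for child spawners.
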(event Custom|ForceCombatParent)

(event Custom|OpenDoor
  (Variables|Referent|SetTempRotDoor (Transformation|GetWorldRotation (Variables|Default|GetRootDoor)))
  (bind _newtrack_0 (Timeline|Timeline PlayFromStart)
    (:Update
      (Transformation|SetWorldRotation (Variables|Default|GetRootDoor) (Math|Rotator|MakeRotator (.roll (Variables|Referent|GetTempRotDoor)) (.pitch (Variables|Referent|GetTempRotDoor)) (Math|Float|Lerp (.yaw (Variables|Referent|GetTempRotDoor)) (+ (.yaw (Variables|Referent|GetTempRotDoor)) (Variables|Referent|GetAnglePorte)) _newtrack_0)) false false))
    (:Finished
      (CallFunction|GoBacktoSpawn))))

(event Custom|GoBackToSpawn)

(fn ConstructionScript)