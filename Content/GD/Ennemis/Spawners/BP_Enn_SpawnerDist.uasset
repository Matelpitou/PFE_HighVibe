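; Spawner for ranged enemies (BP_Enn_Dist) that either pre-spawns them on BeginPlay or spawns them when combat starts.
; A box overlap by BP_PP_Yass or a ForceCombat call triggers combat once, sending enemies to attack.
; Door mode opens the door first, with GoBacktoSpawn resuming staggered spawns at SpawnPoint; otherwise enemies appear at random reachable points within SpawnRadius.
; Spawned enemies register with an optional Arena.
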(event OnComponentBeginOverlap(Box)
  (params (OverlappedComponent :type Primitive%20Component%20Object%20Reference) (OtherActor :type Actor%20Object%20Reference) (OtherComp :type Primitive%20Component%20Object%20Reference) (OtherBodyIndex :type Integer) (bFromSweep :type Boolean) (SweepResult :type Hit%20Result%20Structure%20%28by%20ref%29))
  (if (not (Variables|Spawn|GetDesactiver))
    (Utilities|Casting|CastToBP_PP_Yass OtherActor)
    (Utilities|FlowControl|DoOnce false
      (:Completed
        (if (Variables|Default|GetDoorOrNot)
          (CallFunction|OpenDoor)
          (elif (Variables|Spawn|GetFromBeginning)
            (for _array_element (Variables|Spawn|GetTempEnnSpawned)
              (if (Variables|Spawn|GetLibre)
                (Variables|/Game/GD/Ennemis/Cac/BP_Enn_EnnParent.BP_Enn_EnnParent_C|SetCrazy _array_element true)
                (Default|GoAttack1 _array_element)))
            (elif (Variables|Default|GetDoorOrNot)
              (Variables|Spawn|SetTempVarInt 0)
              (if (< (Variables|Spawn|GetTempVarInt) (Variables|Spawn|GetEnnemiNumber)) :!label _label
                (Math|Integer|IncrementInt (Variables|Spawn|GetTempVarInt)
                  (:%20%20
                    (bind _returnvalue (CallFunction|SpawnEnnDistDoor))
                    (Variables|/Game/GD/Ennemis/Cac/BP_Enn_EnnParent.BP_Enn_EnnParent_C|SetCrazy _returnvalue true)
                    (Variables|/Game/GD/Ennemis/Cac/BP_Enn_EnnParent.BP_Enn_EnnParent_C|SetSystEco _returnvalue (Variables|Referent|GetSystEco))
                    (Default|GoAttack1 _returnvalue)
                    (Utilities|FlowControl|Delay 1.0)
                    (goto _label))))
              (else
                (for _index (range 0 (Variables|Spawn|GetEnnemiNumber))
                  (bind _returnvalue_2 (CallFunction|SpawnEnnDistRandom))
                  (Variables|/Game/GD/Ennemis/Cac/BP_Enn_EnnParent.BP_Enn_EnnParent_C|SetCrazy _returnvalue_2 true)
                  (Variables|/Game/GD/Ennemis/Cac/BP_Enn_EnnParent.BP_Enn_EnnParent_C|SetSystEco _returnvalue_2 (Variables|Referent|GetSystEco))
                  (Default|GoAttack1 _returnvalue_2))))))))))

(event Custom|ForceCombat
  (Utilities|FlowControl|DoOnce false
    (:Completed
      (if (Variables|Default|GetDoorOrNot)
        (CallFunction|OpenDoor)
        (elif (Variables|Spawn|GetFromBeginning)
          (for _array_element (Variables|Spawn|GetTempEnnSpawned)
            (if (Variables|Spawn|GetLibre)
              (Variables|/Game/GD/Ennemis/Cac/BP_Enn_EnnParent.BP_Enn_EnnParent_C|SetCrazy _array_element true)
              (Default|GoAttack1 _array_element)))
          (elif (Variables|Default|GetDoorOrNot)
            (Variables|Spawn|SetTempVarInt 0)
            (if (< (Variables|Spawn|GetTempVarInt) (Variables|Spawn|GetEnnemiNumber)) :!label _label
              (Math|Integer|IncrementInt (Variables|Spawn|GetTempVarInt)
                (:%20%20
                  (bind _returnvalue (CallFunction|SpawnEnnDistDoor))
                  (Variables|/Game/GD/Ennemis/Cac/BP_Enn_EnnParent.BP_Enn_EnnParent_C|SetCrazy _returnvalue true)
                  (Variables|/Game/GD/Ennemis/Cac/BP_Enn_EnnParent.BP_Enn_EnnParent_C|SetSystEco _returnvalue (Variables|Referent|GetSystEco))
                  (Default|GoAttack1 _returnvalue)
                  (Utilities|FlowControl|Delay 1.0)
                  (goto _label))))
            (else
              (for _index (range 0 (Variables|Spawn|GetEnnemiNumber))
                (bind _returnvalue_2 (CallFunction|SpawnEnnDistRandom))
                (Variables|/Game/GD/Ennemis/Cac/BP_Enn_EnnParent.BP_Enn_EnnParent_C|SetCrazy _returnvalue_2 true)
                (Variables|/Game/GD/Ennemis/Cac/BP_Enn_EnnParent.BP_Enn_EnnParent_C|SetSystEco _returnvalue_2 (Variables|Referent|GetSystEco))
                (Default|GoAttack1 _returnvalue_2)))))))))

(event Custom|ForceSpawnTheGuys
  (if (Variables|Default|GetDoorOrNot)
    (Development|SetHiddeninGame (Variables|Default|GetDoor) false false)
    (elif (Variables|Spawn|GetFromBeginning)
      (for _index (range 0 (Variables|Spawn|GetEnnemiNumber))
        (bind _returnvalue (CallFunction|SpawnEnnDistRandom))
        (Utilities|Array|Add (Variables|Spawn|GetTempEnnSpawned) _returnvalue)
        (Variables|/Game/GD/Ennemis/Cac/BP_Enn_EnnParent.BP_Enn_EnnParent_C|SetSystEco _returnvalue (Variables|Referent|GetSystEco))
        (Variables|/Game/GD/Ennemis/Enn_Dist/BP_Enn_Dist.BP_Enn_Dist_C|SetCrowdManager _returnvalue (Variables|Referent|GetReferent))))))

(event EventBeginPlay
  (if (Variables|Spawn|GetTrueSpawnBeginPlay)
    (CallFunction|ForceSpawntheGuys)))

(event EventForceCombatParent
  (CallFunction|ForceCombat))

(event EventGoBacktoSpawn
  (if (Variables|Spawn|GetFromBeginning)
    (for _array_element (Variables|Spawn|GetTempEnnSpawned)
      (if (Variables|Spawn|GetLibre)
        (Variables|/Game/GD/Ennemis/Cac/BP_Enn_EnnParent.BP_Enn_EnnParent_C|SetCrazy _array_element true)
        (Default|GoAttack1 _array_element)))
    (elif (Variables|Default|GetDoorOrNot)
      (Variables|Spawn|SetTempVarInt 0)
      (if (< (Variables|Spawn|GetTempVarInt) (Variables|Spawn|GetEnnemiNumber)) :!label _label
        (Math|Integer|IncrementInt (Variables|Spawn|GetTempVarInt)
          (:%20%20
            (bind _returnvalue (CallFunction|SpawnEnnDistDoor))
            (Variables|/Game/GD/Ennemis/Cac/BP_Enn_EnnParent.BP_Enn_EnnParent_C|SetCrazy _returnvalue true)
            (Variables|/Game/GD/Ennemis/Cac/BP_Enn_EnnParent.BP_Enn_EnnParent_C|SetSystEco _returnvalue (Variables|Referent|GetSystEco))
            (Default|GoAttack1 _returnvalue)
            (Utilities|FlowControl|Delay 1.0)
            (goto _label))))
      (else
        (for _index (range 0 (Variables|Spawn|GetEnnemiNumber))
          (bind _returnvalue_2 (CallFunction|SpawnEnnDistRandom))
          (Variables|/Game/GD/Ennemis/Cac/BP_Enn_EnnParent.BP_Enn_EnnParent_C|SetCrazy _returnvalue_2 true)
          (Variables|/Game/GD/Ennemis/Cac/BP_Enn_EnnParent.BP_Enn_EnnParent_C|SetSystEco _returnvalue_2 (Variables|Referent|GetSystEco))
          (Default|GoAttack1 _returnvalue_2))))))

(fn ConstructionScript)

(fn SpawnEnnDistRandom
  (bind _returnvalue (Transformation|GetActorLocation))
  (bind _arena (Variables|Default|GetArena))
  (bind _spawnradius (Variables|Spawn|GetSpawnRadius))
  (bind _randomlocation (AI|Navigation|GetRandomReachablePointinRadius _returnvalue _spawnradius 0 0))
  (bind _returnvalue_2 (Game|SpawnActorfromClass "/Game/GD/Ennemis/Enn_Dist/BP_Enn_Dist.BP_Enn_Dist_C" (Math|Transform|MakeTransform (Math|Vector|MakeVector (.x _randomlocation) (.y _randomlocation) (+ (.z (Transformation|GetActorLocation)) 1e+01)) "0, 0, 0" "1.000000,1.000000,1.000000") "AdjustIfPossibleButAlwaysSpawn" "MultiplyWithRoot" 0 (Variables|Default|GetNuker) 0))
  (if (Utilities|IsValid _arena)
    (Default|AddEnnemi _arena _returnvalue_2))
  (return _returnvalue_2))

(fn SpawnEnnDistDoor
  (bind _arena (Variables|Default|GetArena))
  (bind _returnvalue (Game|SpawnActorfromClass "/Game/GD/Ennemis/Enn_Dist/BP_Enn_Dist.BP_Enn_Dist_C" (Math|Transform|MakeTransform (Transformation|GetWorldLocation (Variables|Default|GetSpawnPoint)) "0, 0, 0" "1.000000,1.000000,1.000000") "AdjustIfPossibleButAlwaysSpawn" "MultiplyWithRoot" 0 (Variables|Default|GetNuker) 0))
  (if (Utilities|IsValid _arena)
    (Default|AddEnnemi _arena _returnvalue))
  (return _returnvalue))