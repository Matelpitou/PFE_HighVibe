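; Melee enemy spawner that creates BP_Enn_Cac enemies at BeginPlay or when triggered once by BP_PP_Yass overlapping its box or a forced spawn.
; Enemies appear at random reachable points in a radius, or one per second at a door spawn point after OpenDoor and GoBacktoSpawn.
; Libre enemies go Crazy and attack immediately; others reference a crowd manager.
; Each spawn registers with the Arena if valid.
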(event OnComponentBeginOverlap(Box)
  (params (OverlappedComponent :type Primitive%20Component%20Object%20Reference) (OtherActor :type Actor%20Object%20Reference) (OtherComp :type Primitive%20Component%20Object%20Reference) (OtherBodyIndex :type Integer) (bFromSweep :type Boolean) (SweepResult :type Hit%20Result%20Structure%20%28by%20ref%29))
  (bind _doorornot (Variables|Default|GetDoorOrNot))
  (bind _tempennspawned (Variables|Default|GetTempEnnSpawned))
  (bind _libre (Variables|Default|GetLibre))
  ;[1 1 1] Spawn ennemis
  (if (not (Variables|Default|GetDesactiver))
    (Utilities|Casting|CastToBP_PP_Yass OtherActor)
    (Utilities|FlowControl|DoOnce false
      (:Completed
        (if (Variables|Default|GetDoorOrNot)
          (CallFunction|OpenDoor)
          (elif (Variables|Default|GetFromBeginning)
            ;;[1 1 1] Si ennemis pre-existant
            (for _array_element _tempennspawned
              (if _libre
                (Variables|/Game/GD/Ennemis/Cac/BP_Enn_EnnParent.BP_Enn_EnnParent_C|SetCrazy _array_element true)
                (Default|GoAttack1 _array_element)))
            (if (not _libre)
              (Default|AddEnnemis (Variables|Default|GetReferent) _tempennspawned))
            (elif (Variables|Default|GetLibre)
              ;;[1 1 1] Spawn Go Crazy
              (if _doorornot
                (Variables|Default|SetTempVarInt 0)
                (if (< (Variables|Default|GetTempVarInt) (Variables|Default|GetEnnemiNumber)) :!label _label
                  (bind _returnvalue (CallFunction|SpawnEnnCacDoor))
                  (Variables|/Game/GD/Ennemis/Cac/BP_Enn_EnnParent.BP_Enn_EnnParent_C|SetCrazy _returnvalue true)
                  (Variables|/Game/GD/Ennemis/Cac/BP_Enn_EnnParent.BP_Enn_EnnParent_C|SetSystEco _returnvalue (Variables|Default|GetSystEco))
                  (Default|GoAttack1 _returnvalue)
                  (Math|Integer|IncrementInt (Variables|Default|GetTempVarInt)
                    (:%20%20
                      (Utilities|FlowControl|Delay 1.0)
                      (goto _label))))
                (else
                  (for _index (range 0 (Variables|Default|GetEnnemiNumber))
                    (bind _returnvalue_2 (CallFunction|SpawnEnnCacRandom))
                    (Variables|/Game/GD/Ennemis/Cac/BP_Enn_EnnParent.BP_Enn_EnnParent_C|SetCrazy _returnvalue_2 true)
                    (Variables|/Game/GD/Ennemis/Cac/BP_Enn_EnnParent.BP_Enn_EnnParent_C|SetSystEco _returnvalue_2 (Variables|Default|GetSystEco))
                    (Default|GoAttack1 _returnvalue_2))))
              (else
                ;;[1 1 1] Spawn avec crowd manager
                (if _doorornot
                  (Variables|Default|SetTempVarInt 0)
                  (if (< (Variables|Default|GetTempVarInt) (Variables|Default|GetEnnemiNumber)) :!label _label_2
                    (bind _returnvalue_3 (CallFunction|SpawnEnnCacDoor))
                    (Utilities|Array|Add (Variables|Default|GetSpawnedEnnemis) _returnvalue_3)
                    (Variables|/Game/GD/Ennemis/Cac/BP_Enn_Cac.BP_Enn_Cac_C|SetCrowdManager _returnvalue_3 (Variables|Default|GetReferent))
                    (Variables|/Game/GD/Ennemis/Cac/BP_Enn_EnnParent.BP_Enn_EnnParent_C|SetSystEco _returnvalue_3 (Variables|Default|GetSystEco))
                    (Math|Integer|IncrementInt (Variables|Default|GetTempVarInt)
                      (:%20%20
                        (Utilities|FlowControl|Delay 1.0)
                        (goto _label_2))))
                  (else
                    (for _index_2 (range 0 (Variables|Default|GetEnnemiNumber))
                      (bind _returnvalue_4 (CallFunction|SpawnEnnCacRandom))
                      (Utilities|Array|Add (Variables|Default|GetSpawnedEnnemis) _returnvalue_4)
                      (Variables|/Game/GD/Ennemis/Cac/BP_Enn_Cac.BP_Enn_Cac_C|SetCrowdManager _returnvalue_4 (Variables|Default|GetReferent))
                      (Variables|/Game/GD/Ennemis/Cac/BP_Enn_EnnParent.BP_Enn_EnnParent_C|SetSystEco _returnvalue_4 (Variables|Default|GetSystEco)))
                    (Default|AddEnnemis (Variables|Default|GetReferent) (Variables|Default|GetSpawnedEnnemis))))))))))))

(event Custom|ForceSpawn
  (bind _doorornot (Variables|Default|GetDoorOrNot))
  (bind _tempennspawned (Variables|Default|GetTempEnnSpawned))
  (bind _libre (Variables|Default|GetLibre))
  ;[1 1 1] Spawn ennemis
  (Utilities|FlowControl|DoOnce false
    (:Completed
      (if (Variables|Default|GetDoorOrNot)
        (CallFunction|OpenDoor)
        (elif (Variables|Default|GetFromBeginning)
          ;;[1 1 1] Si ennemis pre-existant
          (for _array_element _tempennspawned
            (if _libre
              (Variables|/Game/GD/Ennemis/Cac/BP_Enn_EnnParent.BP_Enn_EnnParent_C|SetCrazy _array_element true)
              (Default|GoAttack1 _array_element)))
          (if (not _libre)
            (Default|AddEnnemis (Variables|Default|GetReferent) _tempennspawned))
          (elif (Variables|Default|GetLibre)
            ;;[1 1 1] Spawn Go Crazy
            (if _doorornot
              (Variables|Default|SetTempVarInt 0)
              (if (< (Variables|Default|GetTempVarInt) (Variables|Default|GetEnnemiNumber)) :!label _label
                (bind _returnvalue (CallFunction|SpawnEnnCacDoor))
                (Variables|/Game/GD/Ennemis/Cac/BP_Enn_EnnParent.BP_Enn_EnnParent_C|SetCrazy _returnvalue true)
                (Variables|/Game/GD/Ennemis/Cac/BP_Enn_EnnParent.BP_Enn_EnnParent_C|SetSystEco _returnvalue (Variables|Default|GetSystEco))
                (Default|GoAttack1 _returnvalue)
                (Math|Integer|IncrementInt (Variables|Default|GetTempVarInt)
                  (:%20%20
                    (Utilities|FlowControl|Delay 1.0)
                    (goto _label))))
              (else
                (for _index (range 0 (Variables|Default|GetEnnemiNumber))
                  (bind _returnvalue_2 (CallFunction|SpawnEnnCacRandom))
                  (Variables|/Game/GD/Ennemis/Cac/BP_Enn_EnnParent.BP_Enn_EnnParent_C|SetCrazy _returnvalue_2 true)
                  (Variables|/Game/GD/Ennemis/Cac/BP_Enn_EnnParent.BP_Enn_EnnParent_C|SetSystEco _returnvalue_2 (Variables|Default|GetSystEco))
                  (Default|GoAttack1 _returnvalue_2))))
            (else
              ;;[1 1 1] Spawn avec crowd manager
              (if _doorornot
                (Variables|Default|SetTempVarInt 0)
                (if (< (Variables|Default|GetTempVarInt) (Variables|Default|GetEnnemiNumber)) :!label _label_2
                  (bind _returnvalue_3 (CallFunction|SpawnEnnCacDoor))
                  (Utilities|Array|Add (Variables|Default|GetSpawnedEnnemis) _returnvalue_3)
                  (Variables|/Game/GD/Ennemis/Cac/BP_Enn_Cac.BP_Enn_Cac_C|SetCrowdManager _returnvalue_3 (Variables|Default|GetReferent))
                  (Variables|/Game/GD/Ennemis/Cac/BP_Enn_EnnParent.BP_Enn_EnnParent_C|SetSystEco _returnvalue_3 (Variables|Default|GetSystEco))
                  (Math|Integer|IncrementInt (Variables|Default|GetTempVarInt)
                    (:%20%20
                      (Utilities|FlowControl|Delay 1.0)
                      (goto _label_2))))
                (else
                  (for _index_2 (range 0 (Variables|Default|GetEnnemiNumber))
                    (bind _returnvalue_4 (CallFunction|SpawnEnnCacRandom))
                    (Utilities|Array|Add (Variables|Default|GetSpawnedEnnemis) _returnvalue_4)
                    (Variables|/Game/GD/Ennemis/Cac/BP_Enn_Cac.BP_Enn_Cac_C|SetCrowdManager _returnvalue_4 (Variables|Default|GetReferent))
                    (Variables|/Game/GD/Ennemis/Cac/BP_Enn_EnnParent.BP_Enn_EnnParent_C|SetSystEco _returnvalue_4 (Variables|Default|GetSystEco)))
                  (Default|AddEnnemis (Variables|Default|GetReferent) (Variables|Default|GetSpawnedEnnemis)))))))))))

(event EventBeginPlay
  ;[1 1 1] Spawn From Beginning
  (if (Variables|Default|GetDoorOrNot)
    (Development|SetHiddeninGame (Variables|Default|GetDoor) false false))
  (if (Variables|Default|GetFromBeginning)
    (for _index (range 0 (Variables|Default|GetEnnemiNumber))
      (bind _returnvalue (CallFunction|SpawnEnnCacRandom))
      (Utilities|Array|Add (Variables|Default|GetTempEnnSpawned) _returnvalue)
      (Variables|/Game/GD/Ennemis/Cac/BP_Enn_EnnParent.BP_Enn_EnnParent_C|SetSystEco _returnvalue (Variables|Default|GetSystEco))
      (Variables|/Game/GD/Ennemis/Cac/BP_Enn_Cac.BP_Enn_Cac_C|SetCrowdManager _returnvalue (Variables|Default|GetReferent)))))

(event EventForceSpawnParent
  ;[1 1 1] Spawn ennemis
  (CallFunction|ForceSpawn))

(event EventGoBacktoSpawn
  (bind _doorornot (Variables|Default|GetDoorOrNot))
  (bind _tempennspawned (Variables|Default|GetTempEnnSpawned))
  (bind _libre (Variables|Default|GetLibre))
  ;[1 1 1] Spawn ennemis
  (if (Variables|Default|GetFromBeginning)
    ;;[1 1 1] Si ennemis pre-existant
    (for _array_element _tempennspawned
      (if _libre
        (Variables|/Game/GD/Ennemis/Cac/BP_Enn_EnnParent.BP_Enn_EnnParent_C|SetCrazy _array_element true)
        (Default|GoAttack1 _array_element)))
    (if (not _libre)
      (Default|AddEnnemis (Variables|Default|GetReferent) _tempennspawned))
    (elif (Variables|Default|GetLibre)
      ;;[1 1 1] Spawn Go Crazy
      (if _doorornot
        (Variables|Default|SetTempVarInt 0)
        (if (< (Variables|Default|GetTempVarInt) (Variables|Default|GetEnnemiNumber)) :!label _label
          (bind _returnvalue (CallFunction|SpawnEnnCacDoor))
          (Variables|/Game/GD/Ennemis/Cac/BP_Enn_EnnParent.BP_Enn_EnnParent_C|SetCrazy _returnvalue true)
          (Variables|/Game/GD/Ennemis/Cac/BP_Enn_EnnParent.BP_Enn_EnnParent_C|SetSystEco _returnvalue (Variables|Default|GetSystEco))
          (Default|GoAttack1 _returnvalue)
          (Math|Integer|IncrementInt (Variables|Default|GetTempVarInt)
            (:%20%20
              (Utilities|FlowControl|Delay 1.0)
              (goto _label))))
        (else
          (for _index (range 0 (Variables|Default|GetEnnemiNumber))
            (bind _returnvalue_2 (CallFunction|SpawnEnnCacRandom))
            (Variables|/Game/GD/Ennemis/Cac/BP_Enn_EnnParent.BP_Enn_EnnParent_C|SetCrazy _returnvalue_2 true)
            (Variables|/Game/GD/Ennemis/Cac/BP_Enn_EnnParent.BP_Enn_EnnParent_C|SetSystEco _returnvalue_2 (Variables|Default|GetSystEco))
            (Default|GoAttack1 _returnvalue_2))))
      (else
        ;;[1 1 1] Spawn avec crowd manager
        (if _doorornot
          (Variables|Default|SetTempVarInt 0)
          (if (< (Variables|Default|GetTempVarInt) (Variables|Default|GetEnnemiNumber)) :!label _label_2
            (bind _returnvalue_3 (CallFunction|SpawnEnnCacDoor))
            (Utilities|Array|Add (Variables|Default|GetSpawnedEnnemis) _returnvalue_3)
            (Variables|/Game/GD/Ennemis/Cac/BP_Enn_Cac.BP_Enn_Cac_C|SetCrowdManager _returnvalue_3 (Variables|Default|GetReferent))
            (Variables|/Game/GD/Ennemis/Cac/BP_Enn_EnnParent.BP_Enn_EnnParent_C|SetSystEco _returnvalue_3 (Variables|Default|GetSystEco))
            (Math|Integer|IncrementInt (Variables|Default|GetTempVarInt)
              (:%20%20
                (Utilities|FlowControl|Delay 1.0)
                (goto _label_2))))
          (else
            (for _index_2 (range 0 (Variables|Default|GetEnnemiNumber))
              (bind _returnvalue_4 (CallFunction|SpawnEnnCacRandom))
              (Utilities|Array|Add (Variables|Default|GetSpawnedEnnemis) _returnvalue_4)
              (Variables|/Game/GD/Ennemis/Cac/BP_Enn_Cac.BP_Enn_Cac_C|SetCrowdManager _returnvalue_4 (Variables|Default|GetReferent))
              (Variables|/Game/GD/Ennemis/Cac/BP_Enn_EnnParent.BP_Enn_EnnParent_C|SetSystEco _returnvalue_4 (Variables|Default|GetSystEco)))
            (Default|AddEnnemis (Variables|Default|GetReferent) (Variables|Default|GetSpawnedEnnemis))))))))

(fn ConstructionScript)

(fn SpawnEnnCacRandom
  (bind _returnvalue (Transformation|GetActorLocation))
  (bind _arena (Variables|Default|GetArena))
  (bind _spawnradius (Variables|Default|GetSpawnRadius))
  (bind _randomlocation (AI|Navigation|GetRandomReachablePointinRadius _returnvalue _spawnradius 0 0))
  (bind _returnvalue_2 (Game|SpawnActorfromClass "/Game/GD/Ennemis/Cac/BP_Enn_Cac.BP_Enn_Cac_C" (Math|Transform|MakeTransform (Math|Vector|MakeVector (.x _randomlocation) (.y _randomlocation) (+ (.z (Transformation|GetActorLocation)) 1e+01)) "0, 0, 0" "1.000000,1.000000,1.000000") "AdjustIfPossibleButAlwaysSpawn" "MultiplyWithRoot" 0 0))
  (if (Utilities|IsValid _arena)
    (Default|AddEnnemi _arena _returnvalue_2))
  (return _returnvalue_2))

(fn SpawnEnnCacDoor
  (bind _arena (Variables|Default|GetArena))
  (bind _returnvalue (Game|SpawnActorfromClass "/Game/GD/Ennemis/Cac/BP_Enn_Cac.BP_Enn_Cac_C" (Math|Transform|MakeTransform (Transformation|GetWorldLocation (Variables|Default|GetSpawnPoint)) "0, 0, 0" "1.000000,1.000000,1.000000") "AdjustIfPossibleButAlwaysSpawn" "MultiplyWithRoot" 0 0))
  (if (Utilities|IsValid _arena)
    (Default|AddEnnemi _arena _returnvalue))
  (return _returnvalue))