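; BP_Element is an enemy-folder Blueprint that appears intended to manage water and electric elements on an actor, but is currently inactive.
; Its SetWater and SetElec events and construction script are empty.
; Disconnected, never-run logic rebuilds the AllWater array by destroying old actors and spawning attached BP_Eau actors.
; That logic staggers their yaw across 90 degrees and gives each the same forward offset.
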(event Custom|SetElec)

(event Custom|SetWater
  (params (NewWaterCount :type Integer)))

(fn ConstructionScript)