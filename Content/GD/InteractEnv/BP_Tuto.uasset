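; One-shot tutorial trigger that pauses the game to show a slideshow when the player enters its box or ForceTuto is called.
; It creates WB_TutoParent with a back-reference, registers it on the game mode, notifies the player and sets time dilation to zero.
; ChangeTuto feeds each AllSlide enum's DT_Tuto row to the widget.
; After the last slide or on EndTuto, it collapses the widget, restores time and destroys itself.
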(event OnComponentBeginOverlap(BoxOverlap)
  (params (OverlappedComponent :type Primitive%20Component%20Object%20Reference) (OtherActor :type Actor%20Object%20Reference) (OtherComp :type Primitive%20Component%20Object%20Reference) (OtherBodyIndex :type Integer) (bFromSweep :type Boolean) (SweepResult :type Hit%20Result%20Structure%20%28by%20ref%29))
  (bind _asbp_pp_yass (Utilities|Casting|CastToBP_PP_Yass OtherActor))
  (Variables|Default|SetPP _asbp_pp_yass)
  (Utilities|FlowControl|DoOnce false
    (:Completed
      (CallFunction|CreateWidget))))

(event Custom|ChangeTuto
  (bind _wb_tuto (Variables|Default|GetWB_Tuto))
  (if (<= (Variables|Default|GetWhichSlide?) (- (Utilities|Array|Length (Variables|Default|GetAllSlide)) 1))
    (bind _returnvalue (Utilities|GetDataTableRow "/Game/GD/UI/Tuto/DT_Tuto.DT_Tuto" (Utilities|String|StringToName (Utilities|String|EnumtoString (Utilities|Array|Get(acopy) (Variables|Default|GetAllSlide) (Variables|Default|GetWhichSlide?)))))
      (:then
        (Variables|/Game/GD/UI/Tuto/WB_TutoParent.WB_TutoParent_C|SetImageTuto _wb_tuto (.Image (Utilities|Struct|BreakStruct_tuto _returnvalue)))
        (Variables|/Game/GD/UI/Tuto/WB_TutoParent.WB_TutoParent_C|SetTextTuto _wb_tuto (.Text (Utilities|Struct|BreakStruct_tuto _returnvalue)))
        (Variables|/Game/GD/UI/Tuto/WB_TutoParent.WB_TutoParent_C|SetDelayChange _wb_tuto (.DelayChange (Utilities|Struct|BreakStruct_tuto _returnvalue)))
        (Default|ChangeSlide _wb_tuto)
        (bind _result (Math|Integer|IncrementInt (Variables|Default|GetWhichSlide?))
          (:%20%20
            (Variables|Default|SetWhichSlide? _result)))))
    (else
      (Widget|SetVisibility (Variables|Default|GetWB_Tuto) "Collapsed")
      (Utilities|Time|SetGlobalTimeDilation 1.0)
      (Default|GoTuto (Variables|Default|GetPP) self)
      (Actor|DestroyActor))))

(event Custom|CreateWidget
  (bind _returnvalue (UserInterface|CreateWidget "/Game/GD/UI/Tuto/WB_TutoParent.WB_TutoParent_C"))
  (bind _output_get (Variables|Default|SetWB_Tuto _returnvalue))
  (Variables|/Game/GD/UI/Tuto/WB_TutoParent.WB_TutoParent_C|SetBP_Tuto _output_get self)
  (UserInterface|Viewport|AddtoViewport _returnvalue 0)
  (bind _asbp_third_person_game_mode (Utilities|Casting|CastToBP_ThirdPersonGameMode (Game|GetGameMode)))
  (Variables|/Game/GD/GameMode/Blueprints/BP_ThirdPersonGameMode.BP_ThirdPersonGameMode_C|SetWidgetActif _asbp_third_person_game_mode (Variables|Default|GetWB_Tuto))
  (Default|GoTuto (Variables|Default|GetPP))
  (Utilities|Time|SetGlobalTimeDilation 0.0)
  (CallFunction|ChangeTuto))

(event Custom|ForceTuto
  (bind _asbp_pp_yass (Utilities|Casting|CastToBP_PP_Yass (Game|GetPlayerCharacter 0)))
  (Variables|Default|SetPP _asbp_pp_yass)
  (Utilities|FlowControl|DoOnce false
    (:Completed
      (CallFunction|CreateWidget))))

(event Custom|EndTuto
  (Widget|SetVisibility (Variables|Default|GetWB_Tuto) "Collapsed")
  (Utilities|Time|SetGlobalTimeDilation 1.0)
  (Default|GoTuto (Variables|Default|GetPP) self)
  (Actor|DestroyActor))

(fn ConstructionScript)