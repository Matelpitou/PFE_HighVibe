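; BP_Env_Caisse is an interactive environment crate that gets knocked away when damaged, then destroys itself.
; Its TakeGamage event applies an impulse to SMActif along the player capsule's forward vector with added upward lift, scaled by ForcePush.
; After a short delay, it spawns the NS_DestroyItem Niagara effect at the mesh's current location and destroys the actor.
; A debug print of the player's forward vector remains in the event.
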(event EventTakeGamage
  (params (Damage :type Integer) (StackEau :type Integer) (StackElec :type Integer))
  (bind _returnvalue (Game|GetPlayerCharacter 0))
  (bind _asbp_pp_yass (Utilities|Casting|CastToBP_PP_Yass _returnvalue))
  (bind _capsulecomponent (Variables|/Script/Engine.Character|GetCapsuleComponent _asbp_pp_yass))
  (bind _returnvalue_2 (Math|Vector|GetForwardVector _capsulecomponent))
  (bind (_x _y _z) (Math|Vector|BreakVector _returnvalue_2))
  (Development|PrintString (Utilities|String|ToString(Vector) _returnvalue_2))
  (Physics|AddImpulse (Variables|Default|GetSM_Actif) (* (Math|Vector|MakeVector _x _y (+ _z 1.0)) (Variables|Default|GetForcePush)) "None" false)
  (Utilities|FlowControl|Delay 4.0)
  (Niagara|SpawnSystematLocation "/Game/GD/InteractEnv/FX_StandBy/NS_DestroyItem.NS_DestroyItem" (Transformation|GetWorldLocation (Variables|Default|GetSM_Actif)) "0, 0, 0" (Math|Conversions|ToVector(Float) (Variables|Default|GetScaleVFX)))
  (Actor|DestroyActor))

(fn ConstructionScript)