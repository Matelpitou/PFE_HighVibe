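; BP_Env_Heal is an environment health pickup for the BP_PP_Yass character.
; It caches BP_MainGameInstance on BeginPlay, which holds Life and LifeMax.
; When Yass overlaps its Box while Life is below LifeMax, it passes DemageTaken to the game instance's Damage function and destroys itself.
; At full life the pickup stays in place.
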(event OnComponentBeginOverlap(Box)
  (params (OverlappedComponent :type Primitive%20Component%20Object%20Reference) (OtherActor :type Actor%20Object%20Reference) (OtherComp :type Primitive%20Component%20Object%20Reference) (OtherBodyIndex :type Integer) (bFromSweep :type Boolean) (SweepResult :type Hit%20Result%20Structure%20%28by%20ref%29))
  (bind _gi (Variables|Default|GetGI))
  (Utilities|Casting|CastToBP_PP_Yass OtherActor)
  (if (< (Variables|/Game/GD/GameMode/Blueprints/BP_MainGameInstance.BP_MainGameInstance_C|GetLife _gi) (Variables|/Game/GD/GameMode/Blueprints/BP_MainGameInstance.BP_MainGameInstance_C|GetLifeMax _gi))
    (Default|Damage (Variables|Default|GetGI) (Variables|Default|GetDemage%20Taken))
    (Actor|DestroyActor)))

(event EventBeginPlay
  (bind _asbp_main_game_instance (Utilities|Casting|CastToBP_MainGameInstance (Game|GetGameInstance)))
  (Variables|Default|SetGI _asbp_main_game_instance))

(fn ConstructionScript)