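; Prototype banter component for BP_PP_Yass that plays sequenced dialogue lines from DT_MainDialogues as debug prints.
; A looping timer event pauses itself, then chains rows by SubStep, waiting each line's duration while its MainStep matches MainDialogueStep.
; When the lookup stops matching, it increments MainDialogueStep and resumes the timer.
; The setup that caches the owner and starts the timer is disconnected from BeginPlay, so the banter never starts by itself.
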(event Custom|Timer
  (Utilities|FlowControl|Delay 0.2)
  (Utilities|Time|PauseTimerbyHandle (Variables|Default|GetDialogueTimer))
  (bind (_out_row_duree_line _returnvalue) (CallFunction|PickOneLine :!label _label))
  (Utilities|FlowControl|Delay _out_row_duree_line)
  (if _returnvalue
    (goto _label)
    (else
      (Math|Integer|IncrementInt (Variables|Default|GetMainDialogueStep)
        (:%20%20
          (Utilities|Time|UnpauseTimerbyHandle (Variables|Default|GetDialogueTimer)))))))

(event EventBeginPlay
  ;[1 1 1] A rebrancher
)

(fn PickOneLine
  (Development|PrintString (Utilities|String|ToString(Float) (Class|KismetSystemLibrary|GetTimerElapsedTimeHandle (Variables|Default|GetDialogueTimer))))
  (bind _returnvalue (Utilities|GetDataTableRow "/Game/GD/PP/Yass/DataDialogues/DT_MainDialogues.DT_MainDialogues" (Utilities|String|StringToName (Utilities|String|ToString(Text) (Utilities|Text|FormatText "WorldDialogue{0}" (Utilities|Text|ToText(Integer) (Variables|Default|GetSubStep))))))
    (:then
      (if (== (.mainstep _returnvalue) (Variables|Default|GetMainDialogueStep))
        (Development|PrintString (Utilities|String|ToString(Text) (.texte _returnvalue)) true true "(R=0.000000,G=0.660000,B=1.000000,A=1.000000)" (.dureeline _returnvalue))
        (Math|Integer|IncrementInt (Variables|Default|GetSubStep)
          (:%20%20
            _)))
      (return (.dureeline _returnvalue) (== (.mainstep _returnvalue) (Variables|Default|GetMainDialogueStep))))))