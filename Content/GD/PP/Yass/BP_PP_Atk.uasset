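; Attack hitbox for the Yass player character, with its Box collision switched on through ActiveCollision.
; On overlap, actors implementing BPI_PP_AtkYass are recorded in a list so each receives only one damage message, carrying damage plus water (Eau) and electric (Elec) stacks.
; A DoOnce lets only the first valid overlap call FreezeTimeAtk on the player's BP_PP_Yass.
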(event OnComponentBeginOverlap(Box)
  (params (OverlappedComponent :type Primitive%20Component%20Object%20Reference) (OtherActor :type Actor%20Object%20Reference) (OtherComp :type Primitive%20Component%20Object%20Reference) (OtherBodyIndex :type Integer) (bFromSweep :type Boolean) (SweepResult :type Hit%20Result%20Structure%20%28by%20ref%29))
  (Variables|Default|SetOther%20Actor OtherActor)
  (if (Utilities|DoesObjectImplementInterface OtherActor "/Game/GD/PP/Yass/BPI_PP_AtkYass.BPI_PP_AtkYass_C")
    (Utilities|FlowControl|Sequence
      (:then_0
        (bind _array_element (Utilities|Array|ForEachLoopwithBreak (Variables|Default|GetListEnnTouch) :!label _label)
          (:LoopBody
            (if (== _array_element (Variables|Default|GetOther%20Actor))
              (Variables|Default|SetExist? true)
              (goto _label Break)))
          (:Completed
            (if (Variables|Default|GetExist?)
              (Variables|Default|SetExist? false)
              (else
                (Utilities|Array|Add (Variables|Default|GetListEnnTouch) (Variables|Default|GetOther%20Actor))
                (Class|BPIPPAtkYass|TakeGamage(Message) (Variables|Default|GetOther%20Actor) (Variables|Default|GetDMG) (Variables|Default|GetStackEau) (Variables|Default|GetStackElec)))))))
      (:then_1
        (Utilities|FlowControl|DoOnce false
          (:Completed
            (bind _asbp_pp_yass (Utilities|Casting|CastToBP_PP_Yass (Game|GetPlayerCharacter 0)))
            (Default|FreezeTimeAtk _asbp_pp_yass)))))))

(fn ConstructionScript)

(fn ActiveCollision
  (Collision|SetCollisionEnabled (Variables|Default|GetBox) "QueryAndPhysics"))