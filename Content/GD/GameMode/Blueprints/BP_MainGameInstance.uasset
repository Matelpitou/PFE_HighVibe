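; Game instance Blueprint that holds the Life and LifeMax values, presumably for the player.
; Damage subtracts the incoming amount, clamps Life between zero and LifeMax, debug-prints the zero check and returns whether Life is depleted.
; AddHpMax reads the AugmentHP row from the DT_PP_Stat data table, adds its Stat to LifeMax and refills Life to the new maximum.
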(fn Damage
  (params (DemageTaken :type Integer))
  (bind _output_get (Variables|Default|SetLife (Math|Float|Clamp(Float) (- (Variables|Default|GetLife) DemageTaken) 0.0 (Variables|Default|GetLifeMax))))
  (Development|PrintString (Utilities|String|ToString(Boolean) (== _output_get 0.0)))
  (if (== _output_get 0.0)
    (return true)
    (else
      (return false))))

(fn AddHpMax
  (bind _returnvalue (Utilities|GetDataTableRow "/Game/GD/PP/Yass/DT_PP_Stat.DT_PP_Stat" "AugmentHP")
    (:then
      (bind _output_get (Variables|Default|SetLifeMax (+ (Variables|Default|GetLifeMax) (Utilities|Struct|BreakStruct_PP_Stat _returnvalue))))
      (Variables|Default|SetLife _output_get))))